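; Player controller that handles shared local input for two players, routing movement and interact input to the PawnPlayer pawns at player indices 0 and 1.
; Per-player axes move pawns on the X/Z plane and, unless move input is ignored, store the last input vector on them.
; Interact actions set a held flag.
; Ctrl+Alt+F triggers the gamemode's door-opening cheat on the tilemap matching the current level index.
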(event EventBeginPlay
  (bind _asmultiplayer_gamemode (Utilities|Casting|CastToMultiplayer_Gamemode (Game|GetGameMode)))
  (Variables|Default|SetGamemode _asmultiplayer_gamemode))

(event EventTick
  (params (DeltaSeconds :type Float%20%28single-precision%29)))

(fn ConstructionScript)

(event Input|ActionEvents|InputActionF
  (params (Key :type Key%20Structure :default "None"))
  (bind _returnvalue (Game|Player|GetPlayerPawn 0))
  (:Pressed
    (bind _aspawn_player (Utilities|Casting|CastToPawnPlayer _returnvalue))
    (Variables|/Game/Blueprints/PawnPlayer.PawnPlayer_C|SetInteract? _aspawn_player true))
  (:Released
    (bind _aspawn_player_2 (Utilities|Casting|CastToPawnPlayer _returnvalue))
    (Variables|/Game/Blueprints/PawnPlayer.PawnPlayer_C|SetInteract? _aspawn_player_2 false)))

(event Input|ActionEvents|InputAction1
  (params (Key :type Key%20Structure :default "None"))
  (bind _returnvalue (Game|Player|GetPlayerPawn 1))
  (:Pressed
    (bind _aspawn_player (Utilities|Casting|CastToPawnPlayer _returnvalue))
    (Variables|/Game/Blueprints/PawnPlayer.PawnPlayer_C|SetInteract? _aspawn_player true))
  (:Released
    (bind _aspawn_player_2 (Utilities|Casting|CastToPawnPlayer _returnvalue))
    (Variables|/Game/Blueprints/PawnPlayer.PawnPlayer_C|SetInteract? _aspawn_player_2 false)))

(event Input|AxisEvents|InputAxisArriba&abajo(1)
  (params (AxisValue :type Float%20%28single-precision%29))
  (bind _aspawn_player (Utilities|Casting|CastToPawnPlayer (Game|Player|GetPlayerPawn 1)))
  (Pawn|Input|AddMovementInput _aspawn_player "0.000000,0.000000,1.000000" AxisValue false)
  (if (not (Class|Controller|IsMoveInputIgnored (Pawn|GetController _aspawn_player)))
    (Variables|/Game/Blueprints/PawnPlayer.PawnPlayer_C|SetArr_Aba%280%29 _aspawn_player (.z (Pawn|Components|PawnMovement|GetLastInputVector (Variables|/Game/Blueprints/PawnPlayer.PawnPlayer_C|GetFloatingPawnMovement1 _aspawn_player))))))

(event Input|AxisEvents|InputAxisIzquierda&derecha(0)
  (params (AxisValue :type Float%20%28single-precision%29))
  (bind _aspawn_player (Utilities|Casting|CastToPawnPlayer (Game|Player|GetPlayerPawn 0)))
  (Pawn|Input|AddMovementInput _aspawn_player "1.000000,0.000000,0.000000" AxisValue false)
  (if (not (Class|Controller|IsMoveInputIgnored (Pawn|GetController _aspawn_player)))
    (Variables|/Game/Blueprints/PawnPlayer.PawnPlayer_C|SetIzq_Der%280%29 _aspawn_player (.x (Pawn|Components|PawnMovement|GetLastInputVector (Variables|/Game/Blueprints/PawnPlayer.PawnPlayer_C|GetFloatingPawnMovement1 _aspawn_player))))))

(event Input|AxisEvents|InputAxisArriba&abajo(0)
  (params (AxisValue :type Float%20%28single-precision%29))
  (bind _aspawn_player (Utilities|Casting|CastToPawnPlayer (Game|Player|GetPlayerPawn 0)))
  (Pawn|Input|AddMovementInput _aspawn_player "0.000000,0.000000,1.000000" AxisValue false)
  (if (not (Class|Controller|IsMoveInputIgnored (Pawn|GetController _aspawn_player)))
    (Variables|/Game/Blueprints/PawnPlayer.PawnPlayer_C|SetArr_Aba%280%29 _aspawn_player (.z (Pawn|Components|PawnMovement|GetLastInputVector (Variables|/Game/Blueprints/PawnPlayer.PawnPlayer_C|GetFloatingPawnMovement1 _aspawn_player))))))

(event Input|AxisEvents|InputAxisIzquierda&derecha(1)
  (params (AxisValue :type Float%20%28single-precision%29))
  (bind _aspawn_player (Utilities|Casting|CastToPawnPlayer (Game|Player|GetPlayerPawn 1)))
  (Pawn|Input|AddMovementInput _aspawn_player "1.000000,0.000000,0.000000" AxisValue false)
  (if (not (Class|Controller|IsMoveInputIgnored (Pawn|GetController _aspawn_player)))
    (Variables|/Game/Blueprints/PawnPlayer.PawnPlayer_C|SetIzq_Der%280%29 _aspawn_player (.x (Pawn|Components|PawnMovement|GetLastInputVector (Variables|/Game/Blueprints/PawnPlayer.PawnPlayer_C|GetFloatingPawnMovement1 _aspawn_player))))))

(event Input|KeyboardEvents|CtrlAltF
  (params (Key :type Key%20Structure :default "None"))
  (bind _gamemode (Variables|Default|GetGamemode))
  (:Pressed
    (switch int (Variables|/Game/Blueprints/Multiplayer_Gamemode.Multiplayer_Gamemode_C|GetLvl%20index (Variables|Default|GetGamemode))
      (:0
        (bind _returnvalue (Actor|GetActorOfClass "/Game/Blueprints/Lvl-Densidad-tilemap_Blueprint.Lvl-Densidad-tilemap_Blueprint_C"))
        (Default|OpenDoorCheat _gamemode (Variables|/Game/Blueprints/Lvl-Densidad-tilemap_Blueprint.Lvl-Densidad-tilemap_Blueprint_C|GetDoors%20to%20break _returnvalue) _returnvalue _gamemode 2))
      (:1
        (bind _returnvalue_2 (Actor|GetActorOfClass "/Game/Blueprints/Lvl-Logica-tilemap_Blueprint.Lvl-Logica-tilemap_Blueprint_C"))
        (Default|OpenDoorCheat _gamemode (Variables|/Game/Blueprints/Lvl-Logica-tilemap_Blueprint.Lvl-Logica-tilemap_Blueprint_C|GetDoors%20to%20break _returnvalue_2) _returnvalue_2 _gamemode 1))
      (:2
        (bind _returnvalue_3 (Actor|GetActorOfClass "/Game/Blueprints/Lvl-Fuerza_y_velocidad_tilemap_Blueprint.Lvl-Fuerza_y_velocidad_tilemap_Blueprint_C"))
        (Default|OpenDoorCheat _gamemode (Variables|/Game/Blueprints/Lvl-Fuerza_y_velocidad_tilemap_Blueprint.Lvl-Fuerza_y_velocidad_tilemap_Blueprint_C|GetDoors%20to%20break _returnvalue_3) _returnvalue_3 _gamemode 1))
      (:3
        (bind _returnvalue_4 (Actor|GetActorOfClass "/Game/Blueprints/Lvl-Mirrors-tilemap_Blueprint.Lvl-Mirrors-tilemap_Blueprint_C"))
        (Default|OpenDoorCheat _gamemode (Variables|/Game/Blueprints/Lvl-Mirrors-tilemap_Blueprint.Lvl-Mirrors-tilemap_Blueprint_C|GetDoors%20to%20break _returnvalue_4) _returnvalue_4 _gamemode 1)))))