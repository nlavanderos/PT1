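; Paper2D tilemap actor for the Mirrors level, which registers interactable buttons for multiplayer and animates scenery tiles.
; BeginPlay makes the map editable, shifts it in Y by its last layer index, resolves button offsets to tile coordinates and sizes press-tracking arrays.
; Button lookup brute-force scans for a specific tile near each position.
; Tick drives a delayed loop that swaps scenery tiles through four frames, locating them through the Gamemode.
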(event EventBeginPlay
  (bind _returnvalue (Transformation|GetActorLocation))
  (bind _object_to_interact_tilemap_ (Variables|Default|GetObject%20to%20interact%28Tilemap%29))
  (bind _returnvalue_2 (Utilities|Array|LastIndex _object_to_interact_tilemap_))
  (bind (_x _y _z) (Math|Vector|BreakVector _returnvalue))
  (Utilities|FlowControl|Sequence
    (:then_0
      (bind _asmultiplayer_gamemode (Utilities|Casting|CastToMultiplayer_Gamemode (Game|GetGameMode)))
      (Variables|Default|SetGamemode _asmultiplayer_gamemode)
      (Class|PaperTileMapComponent|MakeTileMapEditable (Variables|Default|GetRenderComponent)))
    (:then_1
      (Transformation|SetActorLocation (Math|Vector|MakeVector _x (+ _y (Math|Conversions|ToFloat(Integer) (Utilities|Array|LastIndex (Variables|/Script/Paper2D.PaperTileMap|GetTileLayers (Variables|/Script/Paper2D.PaperTileMapComponent|GetTileMap (Variables|Default|GetRenderComponent)))))) _z) false true))
    (:then_2
      ;[1 1 1] Asocia los vectores a sus elementos en el mapa
      (bind (_array_element _array_index) (Utilities|Array|ForEachLoopwithBreak (Variables|Default|GetObject%20to%20interact%28Tilemap%29))
        (:LoopBody
          (bind (_x_2 _y_2) (CallFunction|FindElementonTilemap (+ (Transformation|GetActorLocation) _array_element) (Utilities|Array|LastIndex (Variables|/Script/Paper2D.PaperTileMap|GetTileLayers (Variables|/Script/Paper2D.PaperTileMapComponent|GetTileMap (Variables|Default|GetRenderComponent)))) self))
          (bind _structout (Utilities|Struct|SetmembersinButton_Interaction (Utilities|Struct|MakeButton_Interaction) (+ (Transformation|GetActorLocation) _array_element) _x_2 _y_2))
          (Utilities|Array|SetArrayElem (Variables|Default|GetArray%20of%20Button_Interactions) _array_index _structout true))
        (:Completed
          (for _index (range 0 (* (Variables|/Game/Blueprints/Multiplayer_Gamemode.Multiplayer_Gamemode_C|GetMax_Players (Variables|Default|GetGamemode)) _returnvalue_2))
            (Utilities|Array|SetArrayElem (Variables|Default|GetPresses?%28players%29) _index false true))
          (for _index_2 (range 0 _returnvalue_2)
            (Utilities|Array|SetArrayElem (Variables|Default|GetPresses?%28only%20buttons%29) _index_2 false true)))))))

(event Collision|EventActorBeginOverlap
  (params (OtherActor :type Actor%20Object%20Reference)))

(event EventTick
  (params (DeltaSeconds :type Float%20%28single-precision%29))
  (bind _array (Utilities|Array|MakeArray 124 154 184 214))
  (bind _rendercomponent (Variables|Default|GetRenderComponent))
  (Utilities|FlowControl|Sequence
    (:then_0)
    (:then_1
      ;[1 1 1] Scenery animation
      (bind _index (Utilities|ForLoopwithDelay 0 (Utilities|Array|LastIndex _array) 0.13 :!label _label)
        (:Loop%20Body
          (for _array_element (Variables|Default|GetScenery)
            (bind (_x _y) (Default|FindElementonTilemap(X) (Variables|Default|GetGamemode) _array_element 0 self))
            (Class|PaperTileMapComponent|SetTile _rendercomponent _x _y (Utilities|Array|LastIndex (Variables|/Script/Paper2D.PaperTileMap|GetTileLayers (Variables|/Script/Paper2D.PaperTileMapComponent|GetTileMap _rendercomponent))) (Class|TileMapBlueprintLibrary|MakeTile (Utilities|Array|Get(acopy) _array _index) "/Game/Tileset/minish_chipper_dungeon_03_TileSet.minish_chipper_dungeon_03_TileSet")))
          (goto _label Loop_Body))))))

(fn ConstructionScript)

(fn FindElementonTilemap
  (params (vector :type Vector%20%28by%20ref%29) (integer :type Integer) (Tilemap :type Paper%20Tile%20Map%20Actor%20Object%20Reference))
  (bind _rendercomponent (Variables|Default|GetRenderComponent Tilemap))
  (bind _rendercomponent_2 (Variables|/Script/Paper2D.PaperTileMapActor|GetRenderComponent Tilemap))
  (bind _tilemap (Variables|/Script/Paper2D.PaperTileMapComponent|GetTileMap _rendercomponent))
  (LocalVariables|SetLocal%20Vector%28Find%29 vector)
  (LocalVariables|SetLast_Layer integer)
  (bind _index (Utilities|FlowControl|ForLoopwithBreak 0 (- (Variables|/Script/Paper2D.PaperTileMap|GetMapWidth _tilemap) 1) :!label _label)
    (:LoopBody
      (LocalVariables|SetX%28N%29 _index)
      (bind _index_2 (Utilities|FlowControl|ForLoopwithBreak 0 (- (Variables|/Script/Paper2D.PaperTileMap|GetMapHeight _tilemap) 1))
        (:LoopBody
          (LocalVariables|SetY%28N%29 _index_2)
          (if (and (== (.tileindex (Class|PaperTileMapComponent|GetTile _rendercomponent_2 (LocalVariables|GetX%28N%29) (LocalVariables|GetY%28N%29) (LocalVariables|GetLast_Layer))) 309) (Math|Vector|Equal(Vector) (LocalVariables|GetLocal%20Vector%28Find%29) (Class|PaperTileMapComponent|GetTileCenterPosition _rendercomponent_2 (LocalVariables|GetX%28N%29) (LocalVariables|GetY%28N%29) (LocalVariables|GetLast_Layer) true) 32.0))
            (Utilities|FlowControl|Sequence
              (:then_0
                (bind _output_get (LocalVariables|SetX%28N%29%28aux%29 (LocalVariables|GetX%28N%29)))
                (bind _output_get_2 (LocalVariables|SetY%28N%29%28aux%29 (LocalVariables|GetY%28N%29)))
                (return _output_get _output_get_2))
              (:then_2
                (goto _label Break)))))))))

(fn FindElementonTilemap(X)
  (params (vector :type Vector%20%28by%20ref%29) (integer :type Integer) (Tilemap :type Paper%20Tile%20Map%20Actor%20Object%20Reference))
  (bind _rendercomponent (Variables|Default|GetRenderComponent Tilemap))
  (bind _tilemap (Variables|/Script/Paper2D.PaperTileMapComponent|GetTileMap _rendercomponent))
  (bind _output_get (LocalVariables|SetLocal%20Vector%28Find%29 vector))
  (LocalVariables|SetLast_Layer integer)
  (bind _index (Utilities|FlowControl|ForLoopwithBreak 0 (- (Variables|/Script/Paper2D.PaperTileMap|GetMapWidth _tilemap) 1) :!label _label)
    (:LoopBody
      (LocalVariables|SetX%28N%29 _index)
      (bind _index_2 (Utilities|FlowControl|ForLoopwithBreak 0 (- (Variables|/Script/Paper2D.PaperTileMap|GetMapHeight _tilemap) 1))
        (:LoopBody
          (LocalVariables|SetY%28N%29 _index_2)
          (if (Math|Vector|Equal(Vector) _output_get (Class|PaperTileMapComponent|GetTileCenterPosition (Variables|/Script/Paper2D.PaperTileMapActor|GetRenderComponent Tilemap) (LocalVariables|GetX%28N%29) (LocalVariables|GetY%28N%29) (LocalVariables|GetLast_Layer) true) 16.0)
            (Utilities|FlowControl|Sequence
              (:then_0
                (bind _output_get_2 (LocalVariables|SetX%28N%29%28aux%29 (LocalVariables|GetX%28N%29)))
                (bind _output_get_3 (LocalVariables|SetY%28N%29%28aux%29 (LocalVariables|GetY%28N%29)))
                (return _output_get_2 _output_get_3))
              (:then_1
                (goto _label Break)))))))))