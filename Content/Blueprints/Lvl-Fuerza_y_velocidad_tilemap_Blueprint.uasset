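; Tile map actor Blueprint, apparently for the Fuerza_y_velocidad level, that animates a vertical strip of dungeon tiles.
; On BeginPlay it writes one tile index down part of a single column on layer 1, waits briefly, then writes the adjacent index.
; A Delay wired back to the start repeats the swap endlessly, producing a two-frame flipbook effect through runtime SetTile calls without using Tick.
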(event EventBeginPlay
  (bind _self self)
  (bind _rendercomponent (Variables|Default|GetRenderComponent _self))
  (Utilities|FlowControl|Sequence
    (:then_0
      (for _index (range 3 13) :!label _label
        (Class|PaperTileMapComponent|SetTile _rendercomponent 8 _index 1 (Class|TileMapBlueprintLibrary|MakeTile 291 "/Game/Tileset/minish_chip_dungeon_03_TileSet-LeftSide.minish_chip_dungeon_03_TileSet-LeftSide")))
      (Utilities|FlowControl|Delay 0.2)
      (for _index_2 (range 3 13)
        (Class|PaperTileMapComponent|SetTile _rendercomponent 8 _index_2 1 (Class|TileMapBlueprintLibrary|MakeTile 292 "/Game/Tileset/minish_chip_dungeon_03_TileSet-LeftSide.minish_chip_dungeon_03_TileSet-LeftSide")))
      (Utilities|FlowControl|Delay 0.2)
      (goto _label))))

(event Collision|EventActorBeginOverlap
  (params (OtherActor :type Actor%20Object%20Reference)))

(event EventTick
  (params (DeltaSeconds :type Float%20%28single-precision%29)))

(fn ConstructionScript)