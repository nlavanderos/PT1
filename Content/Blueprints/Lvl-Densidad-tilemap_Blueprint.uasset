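; Paper2D tilemap actor for the density level that turns floor button tiles into pressure plates for Roca actors.
; BeginPlay maps configured offsets to tile coordinates and controlled-object positions in a ButtonInteraction array, caches rocks and makes the map editable.
; Tick compares rock and button positions, updating pressed state and swapping tiles.
; The breakable-door check has no effect; scoring and conveyor-belt animation are disconnected.
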(event EventBeginPlay
  (bind _array_of_button_interactions (Variables|Default|GetArray%20of%20Button_Interactions))
  (Utilities|FlowControl|Sequence
    (:then_0
      ;[1 1 1] Asocia los vectores a sus elementos en el mapa
      (bind (_array_element _array_index) (Utilities|Array|ForEachLoopwithBreak (Variables|Default|GetObject%20to%20interact%28Tilemap%29))
        (:LoopBody
          (bind (_x _y) (CallFunction|FindElementonTilemap (+ (Transformation|GetActorLocation) _array_element) (Utilities|Array|LastIndex (Variables|/Script/Paper2D.PaperTileMap|GetTileLayers (Variables|/Script/Paper2D.PaperTileMapComponent|GetTileMap (Variables|Default|GetRenderComponent)))) self))
          (bind _structout (Utilities|Struct|SetmembersinButton_Interaction (Utilities|Struct|MakeButton_Interaction) (+ (Transformation|GetActorLocation) _array_element) _x _y))
          (Utilities|Array|SetArrayElem _array_of_button_interactions _array_index _structout true))
        (:Completed
          (bind (_array_element_2 _array_index_2) (Utilities|Array|ForEachLoopwithBreak (Variables|Default|GetObject%20to%20control%28Tilemap%29))
            (:LoopBody
              (bind _structout_2 (Utilities|Struct|SetmembersinButton_Interaction (Utilities|Array|Get(acopy) _array_of_button_interactions _array_index_2) (+ _array_element_2 (Transformation|GetActorLocation))))
              (Utilities|Array|SetArrayElem _array_of_button_interactions _array_index_2 _structout_2))))))
    (:then_1
      (bind _outactors (Actor|GetAllActorsOfClass "/Game/Blueprints/Roca.Roca_C"))
      (Variables|Default|SetRocks _outactors))
    (:then_2
      (Class|PaperTileMapComponent|MakeTileMapEditable (Variables|Default|GetRenderComponent)))
    (:then_3
      (bind _asmultiplayer_gamemode (Utilities|Casting|CastToMultiplayer_Gamemode (Game|GetGameMode)))
      (Variables|Default|SetGamemode _asmultiplayer_gamemode))))

(event Collision|EventActorBeginOverlap
  (params (OtherActor :type Actor%20Object%20Reference)))

(event EventTick
  (params (DeltaSeconds :type Float%20%28single-precision%29))
  (bind _returnvalue (Utilities|Select :Index 0 :Option%200 1 :Option%201 0))
  (bind _array_of_button_interactions (Variables|Default|GetArray%20of%20Button_Interactions))
  (bind _rendercomponent (Variables|Default|GetRenderComponent))
  (bind _tilemap (Variables|/Script/Paper2D.PaperTileMapComponent|GetTileMap _rendercomponent))
  (bind _tilelayers (Variables|/Script/Paper2D.PaperTileMap|GetTileLayers _tilemap))
  (bind _returnvalue_2 (Utilities|Array|LastIndex _tilelayers))
  (Utilities|FlowControl|Sequence
    (:then_0
      (Utilities|FlowControl|Delay 0.001)
      ;[1 1 1] Cambia el boton del tilemap apretado a no apretado
      (bind (_array_element _array_index) (Utilities|Array|ForEachLoopwithBreak _array_of_button_interactions)
        (:LoopBody
          (bind _array_element_2 (Utilities|Array|ForEachLoopwithBreak (Variables|Default|GetRocks) :!label _label)
            (:LoopBody
              (if (Math|Vector|Equal(Vector) (Transformation|GetActorLocation _array_element_2) (Utilities|Struct|BreakButton_Interaction _array_element) 16.0)
                (Utilities|FlowControl|Sequence
                  (:then_0
                    (goto _label Break))
                  (:then_1
                    (goto _label_2 Open)))
                (else
                  (Utilities|FlowControl|Sequence
                    (:then_0
                      (bind _structout (Utilities|Struct|SetmembersinButton_Interaction _array_element false))
                      (Utilities|Array|SetArrayElem _array_of_button_interactions _array_index _structout)
                      (Class|PaperTileMapComponent|SetTile _rendercomponent (.xn (Utilities|Array|Get(acopy) _array_of_button_interactions _array_index)) (.yn (Utilities|Array|Get(acopy) _array_of_button_interactions _array_index)) _returnvalue_2 (Utilities|Struct|MakePaperTileInfo 113 "/Game/Tileset/minish_chipper_dungeon_03_TileSet.minish_chipper_dungeon_03_TileSet" false false false)))
                    (:then_1
                      (goto _label_2 Close))))))
            (:Completed
              (Utilities|FlowControl|Gate true :!label _label_2
                (:Exit
                  (bind _structout_2 (Utilities|Struct|SetmembersinButton_Interaction _array_element true))
                  (Utilities|Array|SetArrayElem _array_of_button_interactions _array_index _structout_2)
                  (Class|PaperTileMapComponent|SetTile _rendercomponent (.xn (Utilities|Array|Get(acopy) _array_of_button_interactions _array_index)) (.yn (Utilities|Array|Get(acopy) _array_of_button_interactions _array_index)) _returnvalue_2 (Utilities|Struct|MakePaperTileInfo 143 "/Game/Tileset/minish_chipper_dungeon_03_TileSet.minish_chipper_dungeon_03_TileSet" false false false)))))))))
    (:then_1
      ;[1 1 1] Se agrega puntaje cuando la piedra rompe la puerta
      (for _array_element_3 (Variables|Default|GetDoors%20to%20break)
        (bind (_x _y) (CallFunction|FindElementonTilemap(X) _array_element_3 _returnvalue self))
        (if (and (== (.tileindex (Class|PaperTileMapComponent|GetTile (Variables|Default|GetRenderComponent) _x _y _returnvalue)) 33) (== (.tileset (Class|PaperTileMapComponent|GetTile (Variables|Default|GetRenderComponent) _x _y _returnvalue)) "/Game/Tileset/zelda_tileset_TileSet.zelda_tileset_TileSet"))
          _)))))

(fn ConstructionScript)

(fn FindElementonTilemap
  (params (vector :type Vector%20%28by%20ref%29) (integer :type Integer) (Tilemap :type Paper%20Tile%20Map%20Actor%20Object%20Reference))
  (bind _rendercomponent (Variables|Default|GetRenderComponent Tilemap))
  (bind _rendercomponent_2 (Variables|/Script/Paper2D.PaperTileMapActor|GetRenderComponent Tilemap))
  (bind _tilemap (Variables|/Script/Paper2D.PaperTileMapComponent|GetTileMap _rendercomponent))
  (LocalVariables|SetLocal%20Vector%28Find%29 vector)
  (LocalVariables|SetLast_Layer integer)
  (bind _index (Utilities|FlowControl|ForLoopwithBreak 0 (- (Variables|/Script/Paper2D.PaperTileMap|GetMapWidth _tilemap) 1) :!label _label)
    (:LoopBody
      (LocalVariables|SetX%28N%29 _index)
      (bind _index_2 (Utilities|FlowControl|ForLoopwithBreak 0 (- (Variables|/Script/Paper2D.PaperTileMap|GetMapHeight _tilemap) 1))
        (:LoopBody
          (LocalVariables|SetY%28N%29 _index_2)
          (if (and (== (.tileindex (Class|PaperTileMapComponent|GetTile _rendercomponent_2 (LocalVariables|GetX%28N%29) (LocalVariables|GetY%28N%29) (LocalVariables|GetLast_Layer))) 113) (Math|Vector|Equal(Vector) (LocalVariables|GetLocal%20Vector%28Find%29) (Class|PaperTileMapComponent|GetTileCenterPosition _rendercomponent_2 (LocalVariables|GetX%28N%29) (LocalVariables|GetY%28N%29) (LocalVariables|GetLast_Layer) true) 32.0))
            (Utilities|FlowControl|Sequence
              (:then_0
                (bind _output_get (LocalVariables|SetX%28N%29%28aux%29 (LocalVariables|GetX%28N%29)))
                (bind _output_get_2 (LocalVariables|SetY%28N%29%28aux%29 (LocalVariables|GetY%28N%29)))
                (return _output_get _output_get_2))
              (:then_2
                (goto _label Break)))))))))

(fn FindElementonTilemap(X)
  (params (vector :type Vector%20%28by%20ref%29) (integer :type Integer) (Tilemap :type Paper%20Tile%20Map%20Actor%20Object%20Reference))
  (bind _rendercomponent (Variables|Default|GetRenderComponent Tilemap))
  (bind _tilemap (Variables|/Script/Paper2D.PaperTileMapComponent|GetTileMap _rendercomponent))
  (bind _output_get (LocalVariables|SetLocal%20Vector%28Find%29 vector))
  (LocalVariables|SetLast_Layer integer)
  (bind _index (Utilities|FlowControl|ForLoopwithBreak 0 (- (Variables|/Script/Paper2D.PaperTileMap|GetMapWidth _tilemap) 1) :!label _label)
    (:LoopBody
      (LocalVariables|SetX%28N%29 _index)
      (bind _index_2 (Utilities|FlowControl|ForLoopwithBreak 0 (- (Variables|/Script/Paper2D.PaperTileMap|GetMapHeight _tilemap) 1))
        (:LoopBody
          (LocalVariables|SetY%28N%29 _index_2)
          (if (Math|Vector|Equal(Vector) _output_get (Class|PaperTileMapComponent|GetTileCenterPosition (Variables|/Script/Paper2D.PaperTileMapActor|GetRenderComponent Tilemap) (LocalVariables|GetX%28N%29) (LocalVariables|GetY%28N%29) (LocalVariables|GetLast_Layer) true) 16.0)
            (Utilities|FlowControl|Sequence
              (:then_0
                (bind _output_get_2 (LocalVariables|SetX%28N%29%28aux%29 (LocalVariables|GetX%28N%29)))
                (bind _output_get_3 (LocalVariables|SetY%28N%29%28aux%29 (LocalVariables|GetY%28N%29)))
                (return _output_get_2 _output_get_3))
              (:then_1
                (goto _label Break)))))))))