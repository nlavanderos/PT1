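; Light source actor for a mirror-reflection mechanic that casts a visible beam and starts the reflection chain.
; Tick, with a short Delay, traces forward from its Arrow, ignoring gamemode players.
; Hitting a Mirror's "Box of Reflection" passes it the reflected direction and records it in the shared hit-mirror list; other blocking hits clear both.
; LightRayDraw stretches the LightRay component to the impact point, computing rotation on a fixed-Y plane.
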(event EventBeginPlay
  ;[1 1 1] Light source funcional, envia a espejo
  (Utilities|FlowControl|Sequence
    (:then_0
      (bind _asmultiplayer_gamemode (Utilities|Casting|CastToMultiplayer_Gamemode (Game|GetGameMode)))
      (Variables|Default|SetGamemode _asmultiplayer_gamemode))
    (:then_1
      (bind _asmirror (Utilities|Casting|CastToMirrorClass "/Game/Blueprints/Mirror.Mirror_C"))
      (bind _outactors (Actor|GetAllActorsOfClass _asmirror))
      (bind _output_get (Variables|Default|SetMirrors _outactors))
      (Variables|Default|SetBox%20of%20Reflection (Variables|/Game/Blueprints/Mirror.Mirror_C|GetBox%20of%20Reflection (Utilities|Array|Get(acopy) _output_get))))))

(event Collision|EventActorBeginOverlap
  (params (OtherActor :type Actor%20Object%20Reference)))

(event EventTick
  (params (DeltaSeconds :type Float%20%28single-precision%29))
  (bind _self self)
  ;[1 1 1] Light source funcional, envia a espejo
  (Utilities|FlowControl|Sequence
    (:then_0
      (Utilities|FlowControl|Delay 0.01)
      (Variables|Default|SetLineTrace%28Start%29%28N%29 (Transformation|GetWorldLocation (Variables|Default|GetArrow)))
      (Variables|Default|SetLineTrace%28End%29%28N%29 (Math|Vector|GetForwardVector (Transformation|GetWorldRotation (Variables|Default|GetArrow))))
      (bind (_outhit _returnvalue) (Collision|LineTraceByChannel (Variables|Default|GetLineTrace%28Start%29%28N%29) (+ (Variables|Default|GetLineTrace%28Start%29%28N%29) (* (Variables|Default|GetLineTrace%28End%29%28N%29) 1e+03)) "TraceTypeQuery1" true (Variables|/Game/Blueprints/Multiplayer_Gamemode.Multiplayer_Gamemode_C|GetPlayers%20 (Variables|Default|GetGamemode)) "None" true "(R=1.000000,G=0.000000,B=0.000000,A=1.000000)" "(R=0.000000,G=0.000000,B=0.000000,A=0.000000)" 0.5))
      (Utilities|FlowControl|Sequence
        (:then_0
          (if _returnvalue
            (if (and (== (Utilities|GetClass (.HitActor (Collision|BreakHitResult _outhit))) "/Game/Blueprints/Mirror.Mirror_C") (Utilities|Enum|Equal(Enum) (Utilities|String|GetSubstring (Utilities|GetDisplayName (.HitComponent (Collision|BreakHitResult _outhit))) (Utilities|String|FindSubstring (Utilities|GetDisplayName (.HitComponent (Collision|BreakHitResult _outhit))) "Box of Reflection" false true) (Utilities|String|Len "Box of Reflection")) "Box of Reflection"))
              (Utilities|FlowControl|Sequence
                (:then_0
                  (if (and (!= (Variables|Default|Gethitted%20mirror%28source%29) 0) (== (Variables|Default|Gethitted%20mirror%28source%29) (.HitActor (Collision|BreakHitResult _outhit))))
                    (bind _asmirror (Utilities|Casting|CastToMirror (.HitActor (Collision|BreakHitResult _outhit))))
                    (Variables|/Game/Blueprints/Mirror.Mirror_C|SetOwn%20Normal _asmirror (.ImpactNormal (Collision|BreakHitResult _outhit)))
                    (if (Utilities|Array|IsValidIndex (Variables|/Game/Blueprints/Mirror.Mirror_C|GetMirror_struct_array _asmirror))
                      (bind _structout (Utilities|Struct|SetmembersinMirror_struct (Utilities|Array|Get(acopy) (Variables|/Game/Blueprints/Mirror.Mirror_C|GetMirror_struct_array _asmirror)) (CameraShake|Start (.ImpactPoint (Collision|BreakHitResult _outhit)) (.ImpactPoint (Collision|BreakHitResult _outhit))) (Math|Vector|MirrorVectorbyNormal (Variables|Default|GetLineTrace%28End%29%28N%29) (.ImpactNormal (Collision|BreakHitResult _outhit))) _self true))
                      (Utilities|Array|SetArrayElem (Variables|/Game/Blueprints/Mirror.Mirror_C|GetMirror_struct_array _asmirror) 0 _structout true)
                      (else
                        (bind _structout_2 (Utilities|Struct|SetmembersinMirror_struct (Utilities|Struct|MakeMirror_struct) (CameraShake|Start (.ImpactPoint (Collision|BreakHitResult _outhit)) (.ImpactPoint (Collision|BreakHitResult _outhit))) (Math|Vector|MirrorVectorbyNormal (Variables|Default|GetLineTrace%28End%29%28N%29) (.ImpactNormal (Collision|BreakHitResult _outhit))) _self true))
                        (Utilities|Array|SetArrayElem (Variables|/Game/Blueprints/Mirror.Mirror_C|GetMirror_struct_array _asmirror) 0 _structout_2 true)))
                    (bind _structout_3 (Utilities|Struct|SetmembersinHitted_Mirrors_in_order (Utilities|Struct|MakeHitted_Mirrors_in_order) (Variables|Default|Gethitted%20mirror%28source%29) 0 0 0 self))
                    (Utilities|Array|SetArrayElem (Variables|/Game/Blueprints/Array_of_Hitted_Mirrors.Array_of_Hitted_Mirrors_C|GetArray_of_hitted_mirrors_in_order (Variables|Default|GetArray%20of%20Hitted%20Mirrors)) 0 _structout_3 true)
                    (else
                      (Utilities|FlowControl|Sequence
                        (:then_0
                          (bind _asmirror_2 (Utilities|Casting|CastToMirror (Variables|Default|Gethitted%20mirror%28source%29)))
                          (Utilities|FlowControl|DoOnce false :!label _label
                            (:Completed
                              (bind _structout_4 (Utilities|Struct|SetmembersinMirror_struct (Utilities|Struct|MakeMirror_struct) 0 false))
                              (Utilities|Array|SetArrayElem (Variables|/Game/Blueprints/Mirror.Mirror_C|GetMirror_struct_array _asmirror_2) 0 _structout_4))))
                        (:then_1
                          (goto _label_2 Reset))))))
                (:then_1
                  (Utilities|FlowControl|DoOnce false :!label _label_2
                    (:Completed
                      (Variables|Default|Sethitted%20mirror%28source%29 (.HitActor (Collision|BreakHitResult _outhit))))))
                (:then_2
                  (goto _label Reset)))
              (else
                (Utilities|FlowControl|Sequence
                  (:then_1
                    (for _array_element (Variables|Default|GetMirrors)
                      (Utilities|Array|Clear (Variables|/Game/Blueprints/Mirror.Mirror_C|GetMirror_struct_array _array_element)))
                    (Variables|Default|Sethitted%20mirror%28source%29 0)
                    (Utilities|Array|Clear (Variables|/Game/Blueprints/Array_of_Hitted_Mirrors.Array_of_Hitted_Mirrors_C|GetArray_of_hitted_mirrors_in_order (Variables|Default|GetArray%20of%20Hitted%20Mirrors)))))))))
        (:then_1
          (Rendering|SetVisibility (Variables|Default|GetLight_Ray) (Variables|Default|GetON?) false)
          (CallFunction|LightRayDraw (Variables|Default|GetLineTrace%28Start%29%28N%29) (.ImpactPoint (Collision|BreakHitResult _outhit))))))
    (:then_1
      (bind _asarray_of_hitted_mirrors (Utilities|Casting|CastToArray_of_Hitted_MirrorsClass "/Game/Blueprints/Array_of_Hitted_Mirrors.Array_of_Hitted_Mirrors_C"))
      (bind _outactors (Actor|GetAllActorsOfClass _asarray_of_hitted_mirrors))
      (if (Utilities|Array|IsValidIndex _outactors)
        (Variables|Default|SetArray%20of%20Hitted%20Mirrors (Utilities|Array|Get(acopy) _outactors))))))

(fn ConstructionScript)

(fn LightRayDraw
  (params (Begin :type Vector) (End :type Vector))
  (bind (_x _y _z) (Math|Vector|BreakVector Begin))
  (bind (_x_2 _y_2 _z_2) (Math|Vector|BreakVector End))
  (bind _returnvalue (Math|Vector|Lerp(Vector) Begin End 0.5))
  (bind _returnvalue_2 (Math|Rotator|FindLookatRotation (Math|Vector|MakeVector _x 13.0 _z) (Math|Vector|MakeVector _x_2 13.0 _z_2)))
  (bind (_roll _pitch _yaw) (Math|Rotator|BreakRotator _returnvalue_2))
  (Transformation|SetWorldRotation (Variables|Default|GetLight_Ray) (Math|Rotator|MakeRotator 0.0 (+ _pitch 9e+01) _yaw) false false)
  (Transformation|SetWorldLocation (Variables|Default|GetLight_Ray) (Math|Vector|MakeVector (.x _returnvalue) (.y _returnvalue) (.z _returnvalue)) false false)
  (Transformation|SetWorldScale3D (Variables|Default|GetLight_Ray) (Math|Vector|MakeVector 0.8 1.0 (/ (Math|Vector|VectorLength (- Begin End)) 16.0))))