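; Spring pawn (resorte) for the force-and-speed level that launches overlapping rocks and scores the players' button-triggered use of it.
; Tick matches the spring to pressed tilemap buttons, rewarding launches of normal or gold rocks, penalizing misfires and logging the rock and player over HTTP.
; At a set flipbook frame, a DoOnce, re-armed on reverse playback, applies an arrow-directed impulse scaled by the Tiempo widget's FPS.
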(event EventBeginPlay
  (bind _spring_animation (Variables|Default|GetSpring_Animation))
  (Utilities|IsValid (Game|GetGameMode)
    (:Is%20Valid
      (Utilities|FlowControl|Sequence
        (:then_0
          (bind _asmultiplayer_gamemode (Utilities|Casting|CastToMultiplayer_Gamemode (Game|GetGameMode)))
          (Variables|Default|SetGamemode _asmultiplayer_gamemode))
        (:then_1
          (Components|Timeline|PlayfromStart _spring_animation)
          (Audio|Components|Audio|Stop _spring_animation)
          (Components|Timeline|SetLooping _spring_animation false))))))

(event Collision|EventActorBeginOverlap
  (params (OtherActor :type Actor%20Object%20Reference)))

(event EventTick
  (params (DeltaSeconds :type Float%20%28single-precision%29))
  (bind _gamemode (Variables|Default|GetGamemode))
  (bind _spring_animation (Variables|Default|GetSpring_Animation))
  (bind _overlapbox (Variables|Default|GetOverlapBox))
  (bind _gamemode_2 (Variables|Default|GetGamemode))
  (bind _overlappingactors (Collision|GetOverlappingActors _overlapbox "/Game/Blueprints/Roca.Roca_C" :!class /Script/Engine.PrimitiveComponent))
  (Utilities|IsValid (Variables|Default|GetGamemode)
    (:Is%20Valid
      (Utilities|FlowControl|Sequence
        (:then_0
          (bind _aslvl__fuerza_y_velocidad_tilemap_blueprint (Utilities|Casting|CastToLvl-Fuerza_y_velocidad_tilemap_Blueprint (Variables|/Game/Blueprints/Multiplayer_Gamemode.Multiplayer_Gamemode_C|GetcurrentTileMap (Variables|Default|GetGamemode))))
          (Variables|Default|SetTilemap_4_spring _aslvl__fuerza_y_velocidad_tilemap_blueprint)
          (bind (_array_element _array_index) (Utilities|Array|ForEachLoopwithBreak (Variables|/Game/Blueprints/Lvl-Fuerza_y_velocidad_tilemap_Blueprint.Lvl-Fuerza_y_velocidad_tilemap_Blueprint_C|GetArray%20of%20Button_Interactions _aslvl__fuerza_y_velocidad_tilemap_blueprint))
            (:LoopBody
              (if (.Pressed? (Utilities|Struct|BreakButton_Interaction _array_element))
                (Variables|Default|SetIndex%20True _array_index)
                (if (Math|Vector|Equal(Vector) (Transformation|GetActorLocation) (.Objecttocontrol (Utilities|Struct|BreakButton_Interaction _array_element)) 16.0)
                  (if (Utilities|Array|IsValidIndex _overlappingactors)
                    (bind _asroca (Utilities|Casting|CastToRoca (Utilities|Array|Get(acopy) _overlappingactors)))
                    (if (== (Class|PaperFlipbookComponent|GetPlaybackPositioninFrames _spring_animation) (- (Class|PaperFlipbookComponent|GetFlipbookLengthinFrames _spring_animation) 1))
                      (if (or (Utilities|Enum|Equal(Enum) (Utilities|GetDisplayName (Sprite|GetSprite (Variables|/Game/Blueprints/Roca.Roca_C|GetRocaSprite _asroca))) (Utilities|GetDisplayName (Variables|Default|GetRocaORO))) (Utilities|Enum|Equal(Enum) (Utilities|GetDisplayName (Sprite|GetSprite (Variables|/Game/Blueprints/Roca.Roca_C|GetRocaSprite _asroca))) (Utilities|GetDisplayName (Variables|Default|GetRoca))))
                        (for _array_element_2 (Class|Actor|GetOverlappingComponents)
                          (if (== _array_element_2 (Variables|/Game/Blueprints/Roca.Roca_C|GetOverlap%20Box _asroca))
                            (if (not (Variables|/Game/Blueprints/Multiplayer_Gamemode.Multiplayer_Gamemode_C|GetAll%20true%28doors%20broken%29 (Variables|Default|GetGamemode)))
                              (Utilities|FlowControl|Sequence
                                (:then_0
                                  (Utilities|FlowControl|Delay 0.2)
                                  (Variables|/Game/Blueprints/Multiplayer_Gamemode.Multiplayer_Gamemode_C|Setscore _gamemode (- (Variables|/Game/Blueprints/Multiplayer_Gamemode.Multiplayer_Gamemode_C|Getscore _gamemode) -130)))
                                (:then_1
                                  (for _array_element_3 (Variables|/Game/Blueprints/Multiplayer_Gamemode.Multiplayer_Gamemode_C|GetPlayers%20 (Variables|Default|GetGamemode))
                                    (bind _array_element_4 (Utilities|Array|ForEachLoopwithBreak (Variables|/Game/Blueprints/Lvl-Fuerza_y_velocidad_tilemap_Blueprint.Lvl-Fuerza_y_velocidad_tilemap_Blueprint_C|GetArray%20of%20Button_Interactions _aslvl__fuerza_y_velocidad_tilemap_blueprint) :!label _label)
                                      (:LoopBody
                                        (if (Math|Vector|Equal(Vector) (.button _array_element_4) (Transformation|GetActorLocation _array_element_3) 16.0)
                                          (bind _aspawn_player (Utilities|Casting|CastToPawnPlayer _array_element_3))
                                          (bind _asmy_player_controller (Utilities|Casting|CastToMyPlayerController (Pawn|GetController _aspawn_player)))
                                          (Default|HttpWrite (Variables|Default|GetGamemode) "1" (Utilities|String|Append (Utilities|String|Append "Resorte" (Utilities|GetDisplayName self)) "; " (Utilities|GetDisplayName (Sprite|GetSprite (Variables|/Game/Blueprints/Roca.Roca_C|GetRocaSprite _asroca))) "; " (Utilities|String|ToString(Integer) (Math|Float|Truncate (Physics|GetMass (Variables|/Game/Blueprints/Roca.Roca_C|GetHit/Block%20Box _asroca)))) "; " "Player " (Utilities|String|ToString(Integer) (Class|GameplayStatics|GetPlayerControllerID _asmy_player_controller))))
                                          (goto _label Break))))))))
                            (else
                              (if (Math|Boolean|Equal(Boolean) (Utilities|Array|Get(acopy) (Variables|/Game/Blueprints/Lvl-Fuerza_y_velocidad_tilemap_Blueprint.Lvl-Fuerza_y_velocidad_tilemap_Blueprint_C|GetPressed!%20Copy (Variables|Default|GetTilemap_4_spring)) (Variables|Default|GetIndex%20True)) false)
                                (Utilities|FlowControl|Delay 0.2)
                                (if (not (Variables|/Game/Blueprints/Multiplayer_Gamemode.Multiplayer_Gamemode_C|GetAll%20true%28doors%20broken%29 (Variables|Default|GetGamemode)))
                                  (Variables|/Game/Blueprints/Multiplayer_Gamemode.Multiplayer_Gamemode_C|Setscore _gamemode_2 (- (Variables|/Game/Blueprints/Multiplayer_Gamemode.Multiplayer_Gamemode_C|Getscore _gamemode_2) 30)))))))
                        (else
                          (if (Math|Boolean|Equal(Boolean) (Utilities|Array|Get(acopy) (Variables|/Game/Blueprints/Lvl-Fuerza_y_velocidad_tilemap_Blueprint.Lvl-Fuerza_y_velocidad_tilemap_Blueprint_C|GetPressed!%20Copy (Variables|Default|GetTilemap_4_spring)) (Variables|Default|GetIndex%20True)) false)
                            (Utilities|FlowControl|Delay 0.2)
                            (if (not (Variables|/Game/Blueprints/Multiplayer_Gamemode.Multiplayer_Gamemode_C|GetAll%20true%28doors%20broken%29 (Variables|Default|GetGamemode))) :!label _label_2
                              (Variables|/Game/Blueprints/Multiplayer_Gamemode.Multiplayer_Gamemode_C|Setscore _gamemode_2 (- (Variables|/Game/Blueprints/Multiplayer_Gamemode.Multiplayer_Gamemode_C|Getscore _gamemode_2) 30)))))))
                    (elif (Math|Boolean|Equal(Boolean) (Utilities|Array|Get(acopy) (Variables|/Game/Blueprints/Lvl-Fuerza_y_velocidad_tilemap_Blueprint.Lvl-Fuerza_y_velocidad_tilemap_Blueprint_C|GetPressed!%20Copy2 (Variables|Default|GetTilemap_4_spring)) _array_index) false)
                      (goto _label_2))))))))
        (:then_1
          (if (Class|PaperFlipbookComponent|IsReversing (Variables|Default|GetSpring_Animation))
            (goto _label_3 Reset)
            (elif (== (Class|PaperFlipbookComponent|GetPlaybackPositioninFrames (Variables|Default|GetSpring_Animation)) 3)
              (Utilities|FlowControl|DoOnce false :!label _label_3
                (:Completed
                  (for _array_element_5 (Class|Actor|GetOverlappingComponents)
                    (bind _asroca_2 (Utilities|Casting|CastToRoca (Utilities|Array|Get(acopy) (Collision|GetOverlappingActors "/Game/Blueprints/Roca.Roca_C" :!class /Script/Engine.Actor))))
                    (if (== (Variables|/Game/Blueprints/Roca.Roca_C|GetOverlap%20Box _asroca_2) _array_element_5)
                      (if (Class|SceneComponent|IsAnySimulatingPhysics (Variables|/Game/Blueprints/Roca.Roca_C|GetHit/Block%20Box _asroca_2))
                        (Physics|AddImpulse (Variables|/Game/Blueprints/Roca.Roca_C|GetHit/Block%20Box _asroca_2) (* (Math|Vector|GetForwardVector (Variables|Default|GetArrow)) (* (Variables|Default|GetFPS) 8333.333008)) "None" false)))))))))
        (:then_2
          (bind _foundwidgets (Widget|GetAllWidgetsOfClass "/Game/Widgets/Tiempo.Tiempo_C" false))
          (if (Utilities|Array|IsValidIndex _foundwidgets)
            (Variables|Default|SetFPS (Variables|/Game/Widgets/Tiempo.Tiempo_C|GetFPS (Utilities|Array|Get(acopy) _foundwidgets)))))))))

(event Collision|EventActorEndOverlap
  (params (OtherActor :type Actor%20Object%20Reference)))

(fn ConstructionScript)