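; Player pawn for a multiplayer 2D tilemap puzzle game, with directional flipbooks and a red tint for controller ID 1.
; Tick pushes overlapped rocks on Interact via attachment and impulse, adjusting move speed, and teleports the player back from holes in the force-and-velocity level.
; Each tile change costs score until all true doors are broken.
; Reaching a level-specific exit door stops movement, fades the camera and hides the player.
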(event EventBeginPlay
  (bind _self self)
  (bind (_tilemap_rendercomponent__ _x _y) (|PlayerPositiononTilemap_2 _self))
  (Utilities|FlowControl|Sequence
    (:then_0
      (Utilities|FlowControl|Delay 1e-06)
      (bind _asplayer_controller (Utilities|Casting|CastToPlayerController (Pawn|GetController)))
      (bind _output_get (Variables|Default|SetPlayer%20Controller _asplayer_controller))
      (Utilities|FlowControl|Sequence
        (:then_0
          (Input|EnableInput self (Game|GetPlayerController (Class|GameplayStatics|GetPlayerControllerID _output_get))))
        (:then_1
          (switch int (Class|GameplayStatics|GetPlayerControllerID _output_get)
            (:1
              (Sprite|SetSpriteColor (Variables|Default|GetPlayer_Flipbook) "(R=0.484375,G=0.006752,B=0.000000,A=1.000000)"))))))
    (:then_1
      (bind _asmultiplayer_gamemode (Utilities|Casting|CastToMultiplayer_Gamemode (Game|GetGameMode)))
      (Variables|Default|SetGamemode _asmultiplayer_gamemode))
    (:then_2
      (bind _asmy_game_instance (Utilities|Casting|CastToMyGameInstance (Game|GetGameInstance)))
      (Variables|Default|SetGame%20instance _asmy_game_instance))
    (:then_3
      (Utilities|FlowControl|Delay 1e-06)
      (bind _output_get_2 (Variables|Default|SetX%28pos%29 _x))
      (Variables|Default|SetX%28aux%29 _output_get_2)
      (bind _output_get_3 (Variables|Default|SetY%28pos%29 _y))
      (Variables|Default|SetY%28aux%29 _output_get_3))
    (:then_4
      (Variables|Default|SetVelocity%280%29 1e+02))))

(event Collision|EventActorBeginOverlap
  (params (OtherActor :type Actor%20Object%20Reference)))

(event EventTick
  (params (DeltaSeconds :type Float%20%28single-precision%29))
  (bind _overlappingactors (Collision|GetOverlappingActors "/Game/Blueprints/Roca.Roca_C" :!class /Script/Engine.Actor))
  (bind _self self)
  (bind _gamemode (Variables|Default|GetGamemode))
  (bind _gamemode_2 (Variables|Default|GetGamemode))
  (bind (_tilemap_rendercomponent__ _x _y) (|PlayerPositiononTilemap _self))
  (bind _currenttilemap (Variables|/Game/Blueprints/Multiplayer_Gamemode.Multiplayer_Gamemode_C|GetcurrentTileMap _gamemode_2))
  (Utilities|FlowControl|Sequence
    (:then_0
      (CallFunction|DireccionMov))
    (:then_1
      (bind _aslvl__fuerza_y_velocidad_tilemap_blueprint (Utilities|Casting|CastToLvl-Fuerza_y_velocidad_tilemap_Blueprint _currenttilemap))
      (if (Utilities|Enum|Equal(Enum) (Utilities|GetDisplayName _aslvl__fuerza_y_velocidad_tilemap_blueprint) "Lvl-Fuerza_y_velocidad_tilemap_Blueprint")
        ;[1 1 1] Este tiempo deja pasar a los jugadores con el resorte
        (if (Class|PrimitiveComponent|IsOverlappingComponent (Variables|Default|GetPlayer_Hitbox) (Variables|/Game/Blueprints/Lvl-Fuerza_y_velocidad_tilemap_Blueprint.Lvl-Fuerza_y_velocidad_tilemap_Blueprint_C|GetHole _aslvl__fuerza_y_velocidad_tilemap_blueprint))
          (Utilities|FlowControl|DoOnce false :!label _label
            (:Completed
              (Variables|Default|SetPrevious%20Location (- (- (Transformation|GetActorLocation) (* (Pawn|Components|PawnMovement|GetLastInputVector (Variables|Default|GetFloatingPawnMovement1)) 16.0)) (|Velocity_direction self)))
              (Utilities|FlowControl|Delay 0.2)
              (if (Class|PrimitiveComponent|IsOverlappingComponent (Variables|Default|GetPlayer_Hitbox) (Variables|/Game/Blueprints/Lvl-Fuerza_y_velocidad_tilemap_Blueprint.Lvl-Fuerza_y_velocidad_tilemap_Blueprint_C|GetHole _aslvl__fuerza_y_velocidad_tilemap_blueprint))
                ;[1 1 1] Mueve al jugador a su posicion antes de tocar el agujero
                (Utilities|FlowControl|Delay 0.2)
                (bind _newparam (CallFunction|PositionDifference))
                (Transformation|SetActorLocation _newparam false true)
                (if (Class|PrimitiveComponent|IsOverlappingComponent (Variables|Default|GetPlayer_Hitbox) (Variables|/Game/Blueprints/Lvl-Fuerza_y_velocidad_tilemap_Blueprint.Lvl-Fuerza_y_velocidad_tilemap_Blueprint_C|GetHole _aslvl__fuerza_y_velocidad_tilemap_blueprint))
                  (Transformation|SetActorLocation (|LittleMoreDistance _newparam) false true)))))
          (else
            (goto _label Reset)))))
    (:then_2
      ;[1 1 1] Empujar y tirar
      (if (Utilities|Array|IsValidIndex _overlappingactors)
        (if (Variables|Default|GetInteract?)
          (bind _asroca (Utilities|Casting|CastToRoca (Utilities|Array|Get(acopy) _overlappingactors)))
          (bind _array_element (Utilities|Array|ForEachLoopwithBreak (Class|Actor|GetOverlappingComponents) :!label _label_2)
            (:LoopBody
              (if (== _array_element (Variables|/Game/Blueprints/Roca.Roca_C|GetOverlap%20Box _asroca))
                (Utilities|FlowControl|Sequence
                  (:then_0
                    (goto _label_4 Open))
                  (:then_1
                    (goto _label_2 Break)))
                (else
                  (Utilities|FlowControl|Sequence
                    (:then_0
                      (goto _label_4 Close))
                    (:then_1
                      (bind _output_get (Variables|Default|SetVelocity (Variables|Default|GetVelocity%280%29) :!label _label_3))
                      (Variables|/Script/Engine.FloatingPawnMovement|SetMaxSpeed (Variables|Default|GetFloatingPawnMovement1) _output_get))))))
            (:Completed
              (Utilities|FlowControl|Gate false :!label _label_4
                (:Exit
                  (if (Math|Boolean|ANDBoolean (Class|SceneComponent|IsAnySimulatingPhysics (Variables|/Game/Blueprints/Roca.Roca_C|GetHit/Block%20Box _asroca)) (Variables|Default|GetInteract?) (Class|PrimitiveComponent|IsPhysicsCollisionEnabled (Variables|/Game/Blueprints/Roca.Roca_C|GetHit/Block%20Box _asroca)))
                    (Transformation|AttachActorToActor _asroca self "None" "KeepWorld" "KeepWorld" "KeepWorld" false)
                    (Physics|AddImpulse (Variables|/Game/Blueprints/Roca.Roca_C|GetHit/Block%20Box _asroca) (* (Class|Pawn|GetLastMovementInputVector) 1111.0) "None" false)
                    (Variables|/Script/Engine.FloatingPawnMovement|SetMaxSpeed (Variables|Default|GetFloatingPawnMovement1) (- (Math|Vector|VectorLength (Transformation|GetVelocity _asroca)) 5.0))
                    (else
                      (Transformation|DetachFromActor _asroca "KeepWorld" "KeepWorld" "KeepWorld")
                      (goto _label_3)))))))
          (else
            (goto _label_3)))))
    (:then_3
      (Utilities|FlowControl|Delay 0.0002)
      ;[1 1 1] Determina la posicion del jugador en el Tilemap
      (Utilities|FlowControl|Sequence
        (:then_0
          (bind _output_get_2 (Variables|Default|SetX%28pos%29 _x))
          (Utilities|FlowControl|Delay 0.01)
          (Variables|Default|SetX%28aux%29 _output_get_2))
        (:then_1
          (bind _output_get_3 (Variables|Default|SetY%28pos%29 _y))
          (Utilities|FlowControl|Delay 0.01)
          (Variables|Default|SetY%28aux%29 _output_get_3))
        (:then_2
          (if (!= (Variables|Default|GetX%28pos%29) (Variables|Default|GetX%28aux%29))
            (if (not (Variables|/Game/Blueprints/Multiplayer_Gamemode.Multiplayer_Gamemode_C|GetAll%20true%28doors%20broken%29 _gamemode)) :!label _label_5
              (Variables|/Game/Blueprints/Multiplayer_Gamemode.Multiplayer_Gamemode_C|Setscore _gamemode (- (Variables|/Game/Blueprints/Multiplayer_Gamemode.Multiplayer_Gamemode_C|Getscore _gamemode) 10)))))
        (:then_3
          (if (!= (Variables|Default|GetY%28pos%29) (Variables|Default|GetY%28aux%29))
            (goto _label_5)))))
    (:then_4
      (|PlayeronDoor _currenttilemap))))

(fn ConstructionScript)

(fn DireccionMov
  (bind _player_flipbook (Variables|Default|GetPlayer_Flipbook))
  (if (!= (Variables|/Script/Engine.FloatingPawnMovement|GetMaxSpeed (Variables|Default|GetFloatingPawnMovement1)) 0.0)
    (if (or (!= (Variables|Default|GetArr_Aba%280%29) 0.0) (!= (Variables|Default|GetIzq_Der%280%29) 0.0))
      (Variables|Default|SetDireccions (select (< (Variables|Default|GetIzq_Der%280%29) 0.0) "NewEnumerator0" (select (> (Variables|Default|GetIzq_Der%280%29) 0.0) "NewEnumerator1" (select (> (Variables|Default|GetArr_Aba%280%29) 0.0) "NewEnumerator3" "NewEnumerator2"))))
      (Sprite|SetFlipbook _player_flipbook (Utilities|Select :Index (Variables|Default|GetDireccions) :NewEnumerator0 "/Game/Sprites/PJ_sides/LEFT/Left_mov.Left_mov" :NewEnumerator1 "/Game/Sprites/PJ_sides/RIGHT/Right_mov.Right_mov" :NewEnumerator2 "/Game/Sprites/PJ_sides/DOWN/Down_mov.Down_mov" :NewEnumerator3 "/Game/Sprites/PJ_sides/UP/Up_mov.Up_mov"))
      (else
        (Sprite|SetFlipbook _player_flipbook (Utilities|Select :Index (Variables|Default|GetDireccions) :NewEnumerator0 "/Game/Sprites/PJ_sides/LEFT/L_not_mov.L_not_mov" :NewEnumerator1 "/Game/Sprites/PJ_sides/RIGHT/R_not_mov.R_not_mov" :NewEnumerator2 "/Game/Sprites/PJ_sides/DOWN/D_not_mov.D_not_mov" :NewEnumerator3 "/Game/Sprites/PJ_sides/UP/U_not_mov.U_not_mov") :!label _label)))
    (else
      (goto _label))))

(fn PositionDifference
  (bind _returnvalue (Transformation|GetActorLocation))
  (return (- _returnvalue (- _returnvalue (Variables|Default|GetPrevious%20Location)))))

(fn DissapearPlayer
  (params (NewParam :type Pawn%20Player%20Object%20Reference))
  (bind _player_hitbox (Variables|PawnPlayer_C|GetPlayer_Hitbox NewParam))
  (Rendering|SetVisibility (Variables|PawnPlayer_C|GetPlayer_Flipbook NewParam) false true)
  (Physics|SetSimulatePhysics _player_hitbox false)
  (Collision|SetCollisionEnabled _player_hitbox "NoCollision"))