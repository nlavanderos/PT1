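; Paper2D tilemap actor for a multiplayer dungeon level that runs floor buttons and animated scenery.
; BeginPlay makes the map editable and resolves configured button offsets to tile coordinates.
; Tick detects players by position, comparing against a delayed copy to toggle button tiles and report via Gamemode.HttpWrite until AllTrueDoorsBroken; the overlap-box binding is disconnected.
; Tick also cycles scenery tiles when the Tiempo widget is visible, FPS exceeds a threshold and Effects is on.
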(event Custom|ButtonBox_Overlap
  (params (OverlappedComponent :type Primitive%20Component%20Object%20Reference) (OtherActor :type Actor%20Object%20Reference) (OtherComp :type Primitive%20Component%20Object%20Reference) (OtherBodyIndex :type Integer) (bFromSweep :type Boolean) (SweepResult :type Hit%20Result%20Structure%20%28by%20ref%29))
  (bind _returnvalue (Transformation|GetWorldLocation OverlappedComponent))
  (bind _rendercomponent (Variables|Default|GetRenderComponent))
  (bind _gamemode (Variables|Default|GetGamemode))
  (bind _gamemode_2 (Variables|Default|GetGamemode))
  (bind _tilemap (Variables|/Script/Paper2D.PaperTileMapComponent|GetTileMap _rendercomponent))
  (bind _tilelayers (Variables|/Script/Paper2D.PaperTileMap|GetTileLayers _tilemap))
  (bind _returnvalue_2 (Utilities|Array|LastIndex _tilelayers))
  ;[1 1 1] Cambia el boton del tilemap apretado a no apretado(con evento)
  (if (Math|Boolean|Equal(Boolean) (Utilities|Array|IsValidIndex (Collision|GetOverlappingActors OverlappedComponent "/Game/Blueprints/PawnPlayer.PawnPlayer_C" :!class /Script/Engine.PrimitiveComponent) 1) false)
    (bind (_x _y) (Default|FindElementonTilemap(X) (Variables|Default|GetGamemode) _returnvalue 0 self))
    (Utilities|FlowControl|Delay 0.05)
    (if (== (.tileindex (Class|PaperTileMapComponent|GetTile (Variables|Default|GetRenderComponent) _x _y _returnvalue_2)) 309)
      (Class|PaperTileMapComponent|SetTile (Variables|Default|GetRenderComponent) _x _y _returnvalue_2 (Utilities|Struct|MakePaperTileInfo 279 "/Game/Tileset/minish_chipper_dungeon_03_TileSet.minish_chipper_dungeon_03_TileSet" false false false))
      (if (not (Variables|/Game/Blueprints/Multiplayer_Gamemode.Multiplayer_Gamemode_C|GetAll%20true%28doors%20broken%29 _gamemode))
        (bind (_array_element _array_index) (Utilities|Array|ForEachLoopwithBreak (Variables|Default|GetArray%20of%20Button_Interactions))
          (:LoopBody
            (if (Math|Vector|Equal(Vector) _returnvalue (.button _array_element) 16.0)
              (bind _aspawn_player (Utilities|Casting|CastToPawnPlayer OtherActor))
              (bind _asmy_player_controller (Utilities|Casting|CastToMyPlayerController (Pawn|GetController _aspawn_player)))
              (Default|HttpWrite _gamemode "1" (Utilities|String|Append "Boton" (Utilities|String|ToString(Integer) _array_index) ";" "Set to TRUE; " "Player " (Utilities|String|ToString(Integer) (Class|GameplayStatics|GetPlayerControllerID _asmy_player_controller))))))))
      (else
        (Class|PaperTileMapComponent|SetTile (Variables|Default|GetRenderComponent) _x _y _returnvalue_2 (Utilities|Struct|MakePaperTileInfo 309 "/Game/Tileset/minish_chipper_dungeon_03_TileSet.minish_chipper_dungeon_03_TileSet" false false false))
        (if (not (Variables|/Game/Blueprints/Multiplayer_Gamemode.Multiplayer_Gamemode_C|GetAll%20true%28doors%20broken%29 _gamemode_2))
          (bind (_array_element_2 _array_index_2) (Utilities|Array|ForEachLoopwithBreak (Variables|Default|GetArray%20of%20Button_Interactions))
            (:LoopBody
              (if (Math|Vector|Equal(Vector) _returnvalue (.button _array_element_2) 16.0)
                (bind _aspawn_player_2 (Utilities|Casting|CastToPawnPlayer OtherActor))
                (bind _asmy_player_controller_2 (Utilities|Casting|CastToMyPlayerController (Pawn|GetController _aspawn_player_2)))
                (Default|HttpWrite _gamemode_2 "1" (Utilities|String|Append "Boton" (Utilities|String|ToString(Integer) _array_index_2) ";" "Set to FALSE; " "Player " (Utilities|String|ToString(Integer) (Class|GameplayStatics|GetPlayerControllerID _asmy_player_controller_2))))))))))))

(event EventBeginPlay
  (bind _returnvalue (Transformation|GetActorLocation))
  (bind _object_to_interact_tilemap_ (Variables|Default|GetObject%20to%20interact%28Tilemap%29))
  (bind _returnvalue_2 (Utilities|Array|LastIndex _object_to_interact_tilemap_))
  (bind (_x _y _z) (Math|Vector|BreakVector _returnvalue))
  (Utilities|FlowControl|Sequence
    (:then_0
      (bind _asmultiplayer_gamemode (Utilities|Casting|CastToMultiplayer_Gamemode (Game|GetGameMode)))
      (Variables|Default|SetGamemode _asmultiplayer_gamemode)
      (bind _asmy_game_instance (Utilities|Casting|CastToMyGameInstance (Game|GetGameInstance)))
      (Variables|Default|SetGame%20instance _asmy_game_instance)
      (Class|PaperTileMapComponent|MakeTileMapEditable (Variables|Default|GetRenderComponent)))
    (:then_1
      (Transformation|SetActorLocation (Math|Vector|MakeVector _x (+ _y (Math|Conversions|ToFloat(Integer) (Utilities|Array|LastIndex (Variables|/Script/Paper2D.PaperTileMap|GetTileLayers (Variables|/Script/Paper2D.PaperTileMapComponent|GetTileMap (Variables|Default|GetRenderComponent)))))) _z) false true))
    (:then_2
      ;[1 1 1] Asocia los vectores a sus elementos en el mapa
      (bind (_array_element _array_index) (Utilities|Array|ForEachLoopwithBreak (Variables|Default|GetObject%20to%20interact%28Tilemap%29))
        (:LoopBody
          (bind (_x_2 _y_2) (CallFunction|FindElementonTilemap (+ (Transformation|GetActorLocation) _array_element) (Utilities|Array|LastIndex (Variables|/Script/Paper2D.PaperTileMap|GetTileLayers (Variables|/Script/Paper2D.PaperTileMapComponent|GetTileMap (Variables|Default|GetRenderComponent)))) self))
          (bind _structout (Utilities|Struct|SetmembersinButton_Interaction (Utilities|Struct|MakeButton_Interaction) (+ (Transformation|GetActorLocation) _array_element) _x_2 _y_2))
          (Utilities|Array|SetArrayElem (Variables|Default|GetArray%20of%20Button_Interactions) _array_index _structout true))
        (:Completed
          (for _index (range 0 (* (Variables|/Game/Blueprints/Multiplayer_Gamemode.Multiplayer_Gamemode_C|GetMax_Players (Variables|Default|GetGamemode)) _returnvalue_2))
            (Utilities|Array|SetArrayElem (Variables|Default|GetPresses?%28players%29) _index false true))
          (for _index_2 (range 0 _returnvalue_2)
            (Utilities|Array|SetArrayElem (Variables|Default|GetPresses?%28only%20buttons%29) _index_2 false true)))))))

(event Collision|EventActorBeginOverlap
  (params (OtherActor :type Actor%20Object%20Reference)))

(event EventTick
  (params (DeltaSeconds :type Float%20%28single-precision%29))
  (bind _array (Utilities|Array|MakeArray 124 154 184 214))
  (bind _array_of_button_interactions (Variables|Default|GetArray%20of%20Button_Interactions))
  (bind _rendercomponent (Variables|Default|GetRenderComponent))
  (bind _rendercomponent_2 (Variables|Default|GetRenderComponent))
  (bind _rendercomponent_3 (Variables|Default|GetRenderComponent))
  (bind _gamemode (Variables|Default|GetGamemode))
  (bind _gamemode_2 (Variables|Default|GetGamemode))
  (bind _tilemap (Variables|/Script/Paper2D.PaperTileMapComponent|GetTileMap _rendercomponent))
  (bind _tilelayers (Variables|/Script/Paper2D.PaperTileMap|GetTileLayers _tilemap))
  (bind _returnvalue (Utilities|Array|LastIndex _tilelayers))
  (Utilities|FlowControl|Sequence
    (:then_0
      (Utilities|FlowControl|Sequence
        (:then_0
          ;[1 1 1] Cambia el boton del tilemap apretado a no apretado(no en uso)
          (bind (_array_element _array_index) (Utilities|Array|ForEachLoopwithBreak (Variables|Default|GetArray%20of%20Button_Interactions))
            (:LoopBody
              (Variables|Default|Setindex_aux _array_index)
              (bind _index (Utilities|FlowControl|ForLoopwithBreak 0 (Utilities|Array|LastIndex (Variables|/Game/Blueprints/Multiplayer_Gamemode.Multiplayer_Gamemode_C|GetPlayers%20 (Variables|Default|GetGamemode))) :!label _label)
                (:LoopBody
                  (Utilities|FlowControl|Sequence
                    (:then_0
                      (if (Math|Vector|Equal(Vector) (Transformation|GetActorLocation (Utilities|Array|Get(acopy) (Variables|/Game/Blueprints/Multiplayer_Gamemode.Multiplayer_Gamemode_C|GetPlayers%20 (Variables|Default|GetGamemode)) _index)) (Utilities|Struct|BreakButton_Interaction _array_element) 16.0)
                        (Variables|Default|Setindex_aux_true (Variables|Default|Getindex_aux))
                        (Utilities|FlowControl|Sequence
                          (:then_0
                            (bind _structout (Utilities|Struct|SetmembersinButton_Interaction _array_element true))
                            (Utilities|Array|SetArrayElem _array_of_button_interactions (Variables|Default|Getindex_aux_true) _structout)
                            (Utilities|Array|SetArrayElem (Variables|Default|GetPresses?%28only%20buttons%29) (Variables|Default|Getindex_aux_true) true))
                          (:then_1
                            (goto _label Break)))
                        (elif (Math|Boolean|Equal(Boolean) (.pressed? (Utilities|Array|Get(acopy) (Variables|Default|GetArray%20of%20Button_Interactions) (Variables|Default|Getindex_aux))) true)
                          (bind _structout_2 (Utilities|Struct|SetmembersinButton_Interaction _array_element false))
                          (Utilities|Array|SetArrayElem _array_of_button_interactions (Variables|Default|Getindex_aux) _structout_2)
                          (Utilities|Array|SetArrayElem (Variables|Default|GetPresses?%28only%20buttons%29) (Variables|Default|Getindex_aux) false))))))))
            (:Completed
              (Utilities|FlowControl|Delay 1e-05)
              (Variables|Default|SetPresses?%28only%20buttons%20copy%29 (Variables|Default|GetPresses?%28only%20buttons%29)))))
        (:then_1
          (for (_array_element_2 _array_index_2) (Variables|Default|GetArray%20of%20Button_Interactions)
            (if (.pressed? _array_element_2)
              (if (Math|Boolean|Equal(Boolean) (Utilities|Array|Get(acopy) (Variables|Default|GetPresses?%28only%20buttons%20copy%29) _array_index_2) false)
                (if (== (.tileindex (Class|PaperTileMapComponent|GetTile _rendercomponent_2 (.xn (Utilities|Array|Get(acopy) (Variables|Default|GetArray%20of%20Button_Interactions) _array_index_2)) (.yn (Utilities|Array|Get(acopy) (Variables|Default|GetArray%20of%20Button_Interactions) _array_index_2)) (Utilities|Array|LastIndex (Variables|/Script/Paper2D.PaperTileMap|GetTileLayers (Variables|/Script/Paper2D.PaperTileMapComponent|GetTileMap _rendercomponent_2))))) 309)
                  (Class|PaperTileMapComponent|SetTile _rendercomponent (.xn (Utilities|Array|Get(acopy) (Variables|Default|GetArray%20of%20Button_Interactions) _array_index_2)) (.yn (Utilities|Array|Get(acopy) (Variables|Default|GetArray%20of%20Button_Interactions) _array_index_2)) _returnvalue (Utilities|Struct|MakePaperTileInfo 279 "/Game/Tileset/minish_chipper_dungeon_03_TileSet.minish_chipper_dungeon_03_TileSet" false false false))
                  (if (not (Variables|/Game/Blueprints/Multiplayer_Gamemode.Multiplayer_Gamemode_C|GetAll%20true%28doors%20broken%29 _gamemode))
                    (bind (_array_element_3 _array_index_3) (Utilities|Array|ForEachLoopwithBreak (Variables|Default|GetArray%20of%20Button_Interactions))
                      (:LoopBody
                        (bind _array_element_4 (Utilities|Array|ForEachLoopwithBreak (Variables|/Game/Blueprints/Multiplayer_Gamemode.Multiplayer_Gamemode_C|GetPlayers%20 _gamemode) :!label _label_2)
                          (:LoopBody
                            (if (Math|Vector|Equal(Vector) (.button _array_element_3) (Transformation|GetActorLocation _array_element_4) 16.0)
                              (goto _label_2 Break)))
                          (:Completed
                            (bind _aspawn_player (Utilities|Casting|CastToPawnPlayer _array_element_4))
                            (bind _asmy_player_controller (Utilities|Casting|CastToMyPlayerController (Pawn|GetController _aspawn_player)))
                            (Default|HttpWrite _gamemode "1" (Utilities|String|Append "Boton" (Utilities|String|ToString(Integer) _array_index_3) ";" "Set to TRUE; " "Player " (Utilities|String|ToString(Integer) (Class|GameplayStatics|GetPlayerControllerID _asmy_player_controller)))))))))
                  (else
                    (Class|PaperTileMapComponent|SetTile _rendercomponent (.xn (Utilities|Array|Get(acopy) (Variables|Default|GetArray%20of%20Button_Interactions) _array_index_2)) (.yn (Utilities|Array|Get(acopy) (Variables|Default|GetArray%20of%20Button_Interactions) _array_index_2)) _returnvalue (Utilities|Struct|MakePaperTileInfo 309 "/Game/Tileset/minish_chipper_dungeon_03_TileSet.minish_chipper_dungeon_03_TileSet" false false false))
                    (if (not (Variables|/Game/Blueprints/Multiplayer_Gamemode.Multiplayer_Gamemode_C|GetAll%20true%28doors%20broken%29 _gamemode_2))
                      (bind (_array_element_5 _array_index_4) (Utilities|Array|ForEachLoopwithBreak (Variables|Default|GetArray%20of%20Button_Interactions))
                        (:LoopBody
                          (bind _array_element_6 (Utilities|Array|ForEachLoopwithBreak (Variables|/Game/Blueprints/Multiplayer_Gamemode.Multiplayer_Gamemode_C|GetPlayers%20 _gamemode_2) :!label _label_3)
                            (:LoopBody
                              (if (Math|Vector|Equal(Vector) (.button _array_element_5) (Transformation|GetActorLocation _array_element_6) 16.0)
                                (goto _label_3 Break)))
                            (:Completed
                              (bind _aspawn_player_2 (Utilities|Casting|CastToPawnPlayer _array_element_6))
                              (bind _asmy_player_controller_2 (Utilities|Casting|CastToMyPlayerController (Pawn|GetController _aspawn_player_2)))
                              (Default|HttpWrite _gamemode_2 "1" (Utilities|String|Append "Boton" (Utilities|String|ToString(Integer) _array_index_4) ";" "Set to FALSE; " "Player " (Utilities|String|ToString(Integer) (Class|GameplayStatics|GetPlayerControllerID _asmy_player_controller_2)))))))))))))))))
    (:then_1
      ;[1 1 1] Scenery animation
      (bind _foundwidgets (Widget|GetAllWidgetsOfClass "/Game/Widgets/Tiempo.Tiempo_C" false))
      (if (and (Widget|IsVisible (Utilities|Array|Get(acopy) _foundwidgets)) (Utilities|Array|IsValidIndex _foundwidgets))
        (if (and (> (Variables|/Game/Widgets/Tiempo.Tiempo_C|GetFPS (Utilities|Array|Get(acopy) _foundwidgets)) 29.0) (Variables|/Game/Blueprints/MyGameInstance.MyGameInstance_C|GetEffects? (Variables|Default|GetGame%20instance)))
          (bind _index_2 (Utilities|ForLoopwithDelay 0 (Utilities|Array|LastIndex _array) 0.13 :!label _label_4)
            (:Loop%20Body
              (for _array_element_7 (Variables|Default|GetScenery)
                (bind (_x _y) (Default|FindElementonTilemap(X) (Variables|Default|GetGamemode) _array_element_7 0 self))
                (Class|PaperTileMapComponent|SetTile _rendercomponent_3 _x _y (Utilities|Array|LastIndex (Variables|/Script/Paper2D.PaperTileMap|GetTileLayers (Variables|/Script/Paper2D.PaperTileMapComponent|GetTileMap _rendercomponent_3))) (Class|TileMapBlueprintLibrary|MakeTile (Utilities|Array|Get(acopy) _array _index_2) "/Game/Tileset/minish_chipper_dungeon_03_TileSet.minish_chipper_dungeon_03_TileSet")))
              (goto _label_4 Loop_Body))))))))

(fn ConstructionScript)

(fn FindElementonTilemap
  (params (vector :type Vector%20%28by%20ref%29) (integer :type Integer) (Tilemap :type Paper%20Tile%20Map%20Actor%20Object%20Reference))
  (bind _rendercomponent (Variables|Default|GetRenderComponent Tilemap))
  (bind _rendercomponent_2 (Variables|/Script/Paper2D.PaperTileMapActor|GetRenderComponent Tilemap))
  (bind _tilemap (Variables|/Script/Paper2D.PaperTileMapComponent|GetTileMap _rendercomponent))
  (LocalVariables|SetLocal%20Vector%28Find%29 vector)
  (LocalVariables|SetLast_Layer integer)
  (bind _index (Utilities|FlowControl|ForLoopwithBreak 0 (- (Variables|/Script/Paper2D.PaperTileMap|GetMapWidth _tilemap) 1) :!label _label)
    (:LoopBody
      (LocalVariables|SetX%28N%29 _index)
      (bind _index_2 (Utilities|FlowControl|ForLoopwithBreak 0 (- (Variables|/Script/Paper2D.PaperTileMap|GetMapHeight _tilemap) 1))
        (:LoopBody
          (LocalVariables|SetY%28N%29 _index_2)
          (if (and (== (.tileindex (Class|PaperTileMapComponent|GetTile _rendercomponent_2 (LocalVariables|GetX%28N%29) (LocalVariables|GetY%28N%29) (LocalVariables|GetLast_Layer))) 309) (Math|Vector|Equal(Vector) (LocalVariables|GetLocal%20Vector%28Find%29) (Class|PaperTileMapComponent|GetTileCenterPosition _rendercomponent_2 (LocalVariables|GetX%28N%29) (LocalVariables|GetY%28N%29) (LocalVariables|GetLast_Layer) true) 32.0))
            (Utilities|FlowControl|Sequence
              (:then_0
                (bind _output_get (LocalVariables|SetX%28N%29%28aux%29 (LocalVariables|GetX%28N%29)))
                (bind _output_get_2 (LocalVariables|SetY%28N%29%28aux%29 (LocalVariables|GetY%28N%29)))
                (return _output_get _output_get_2))
              (:then_2
                (goto _label Break)))))))))

(fn FindElementonTilemap(X)
  (params (vector :type Vector%20%28by%20ref%29) (integer :type Integer) (Tilemap :type Paper%20Tile%20Map%20Actor%20Object%20Reference))
  (bind _rendercomponent (Variables|Default|GetRenderComponent Tilemap))
  (bind _tilemap (Variables|/Script/Paper2D.PaperTileMapComponent|GetTileMap _rendercomponent))
  (bind _output_get (LocalVariables|SetLocal%20Vector%28Find%29 vector))
  (LocalVariables|SetLast_Layer integer)
  (bind _index (Utilities|FlowControl|ForLoopwithBreak 0 (- (Variables|/Script/Paper2D.PaperTileMap|GetMapWidth _tilemap) 1) :!label _label)
    (:LoopBody
      (LocalVariables|SetX%28N%29 _index)
      (bind _index_2 (Utilities|FlowControl|ForLoopwithBreak 0 (- (Variables|/Script/Paper2D.PaperTileMap|GetMapHeight _tilemap) 1))
        (:LoopBody
          (LocalVariables|SetY%28N%29 _index_2)
          (if (Math|Vector|Equal(Vector) _output_get (Class|PaperTileMapComponent|GetTileCenterPosition (Variables|/Script/Paper2D.PaperTileMapActor|GetRenderComponent Tilemap) (LocalVariables|GetX%28N%29) (LocalVariables|GetY%28N%29) (LocalVariables|GetLast_Layer) true) 16.0)
            (Utilities|FlowControl|Sequence
              (:then_0
                (bind _output_get_2 (LocalVariables|SetX%28N%29%28aux%29 (LocalVariables|GetX%28N%29)))
                (bind _output_get_3 (LocalVariables|SetY%28N%29%28aux%29 (LocalVariables|GetY%28N%29)))
                (return _output_get_2 _output_get_3))
              (:then_1
                (goto _label Break)))))))))