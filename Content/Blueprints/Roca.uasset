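; Pushable-style physics rock for the force and velocity (Fuerza y velocidad) tilemap level.
; On BeginPlay its sprite variant (plain, steel, gold, diamond) sets mass and a Radio value, both copied to an Actor_Stats widget.
; Hitting the tilemap zeroes its velocity, and staying in the tilemap's Hole briefly teleports it back to its start location.
; Tick polls overlaps for that reset and shows the widget only while the player overlaps.
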(event OnComponentHit(Hit/BlockBox)
  (params (HitComponent :type Primitive%20Component%20Object%20Reference) (OtherActor :type Actor%20Object%20Reference) (OtherComp :type Primitive%20Component%20Object%20Reference) (NormalImpulse :type Vector :default "0, 0, 0") (Hit :type Hit%20Result%20Structure%20%28by%20ref%29))
  (if (== OtherActor (Variables|Default|GetTilemap%20Reference))
    (Physics|SetPhysicsLinearVelocity (Variables|Default|GetHit/Block%20Box) "0, 0, 0" false "None")))

(event EventBeginPlay
  (bind _hit_block_box (Variables|Default|GetHit/Block%20Box))
  (Utilities|FlowControl|Sequence
    (:then_0
      (bind _aslvl__fuerza_y_velocidad_tilemap_blueprint (Utilities|Casting|CastToLvl-Fuerza_y_velocidad_tilemap_BlueprintClass "/Game/Blueprints/Lvl-Fuerza_y_velocidad_tilemap_Blueprint.Lvl-Fuerza_y_velocidad_tilemap_Blueprint_C"))
      (bind _returnvalue (Actor|GetActorOfClass _aslvl__fuerza_y_velocidad_tilemap_blueprint))
      (Variables|Default|SetTileMap%20Reference _returnvalue))
    (:then_1
      (Variables|Default|SetPrevious%20Location (Transformation|GetActorLocation)))
    (:then_2
      (bind _asactor_stats (Utilities|Casting|CastToActor_Stats (UserInterface|GetUserWidgetObject (Variables|Default|GetWidgetComponent))))
      (Variables|Default|SetWidget _asactor_stats))
    (:then_3
      (switch string (Utilities|GetDisplayName (Sprite|GetSprite (Variables|Default|GetRocaSprite)))
        (:roca_Sprite
          (Class|PrimitiveComponent|SetMassOverrideinKg _hit_block_box "None" 3e+01 true)
          (Variables|Default|SetRadio%28N%29 0.6))
        (:rocaAcero_Sprite
          (Class|PrimitiveComponent|SetMassOverrideinKg _hit_block_box "None" 7e+01 true)
          (Variables|Default|SetRadio%28N%29 0.15))
        (:rocaOro_Sprite
          (Class|PrimitiveComponent|SetMassOverrideinKg _hit_block_box "None" 5e+01 true)
          (Variables|Default|SetRadio%28N%29 0.5))
        (:rocaDiamante_Sprite
          (Class|PrimitiveComponent|SetMassOverrideinKg _hit_block_box "None" 1e+02 true)
          (Variables|Default|SetRadio%28N%29 0.3)))
      (Variables|/Game/Widgets/Actor_Stats.Actor_Stats_C|SetRadio (Variables|Default|GetWidget) (Variables|Default|GetRadio%28N%29))
      (Variables|/Game/Widgets/Actor_Stats.Actor_Stats_C|SetMass (Variables|Default|GetWidget) (Physics|GetMass (Variables|Default|GetHit/Block%20Box)))
      (Widget|SetVisibility (Variables|Default|GetWidget) "Hidden"))))

(event Collision|EventActorBeginOverlap
  (params (OtherActor :type Actor%20Object%20Reference)))

(event EventTick
  (params (DeltaSeconds :type Float%20%28single-precision%29))
  (bind _widget (Variables|Default|GetWidget))
  (bind _tilemap_reference (Variables|Default|GetTileMap%20Reference))
  (bind _overlap_box (Variables|Default|GetOverlap%20Box))
  (bind _hole (Variables|/Game/Blueprints/Lvl-Fuerza_y_velocidad_tilemap_Blueprint.Lvl-Fuerza_y_velocidad_tilemap_Blueprint_C|GetHole _tilemap_reference))
  (bind _returnvalue (Class|PrimitiveComponent|IsOverlappingComponent _overlap_box _hole))
  (Utilities|FlowControl|Sequence
    (:then_0
      ;[1 1 1] Devuelve a la piedra a su posicion original si esta en el agujero/hole
      (if (Utilities|Enum|Equal(Enum) (Utilities|GetDisplayName _tilemap_reference) "Lvl-Fuerza_y_velocidad_tilemap_Blueprint")
        (if _returnvalue
          (Utilities|FlowControl|DoOnce false :!label _label
            (:Completed
              (Utilities|FlowControl|Delay 0.2)
              (if _returnvalue
                (Utilities|FlowControl|Delay 0.2)
                (Transformation|SetActorLocation (Variables|Default|GetPrevious%20Location) false true))))
          (else
            (goto _label Reset)))))
    (:then_1
      (if (Utilities|Array|IsValidIndex (Collision|GetOverlappingActors (Variables|Default|GetOverlap%20Box) "/Game/Blueprints/PawnPlayer.PawnPlayer_C" :!class /Script/Engine.PrimitiveComponent))
        (Widget|SetVisibility _widget "Visible")
        (else
          (Widget|SetVisibility _widget "Hidden"))))))

(fn ConstructionScript)