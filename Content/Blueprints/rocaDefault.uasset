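; Default rock actor (roca) with a physics-driven sprite that stops when it hits the level's tilemap.
; On BeginPlay it casts to the Lvl-Fuerza_y_velocidad tilemap Blueprint and stores a found actor as TilemapReference.
; When HitBlockBox hits that actor, the RenderComponent's linear velocity is zeroed.
; Tick only reads velocity; debug prints for velocity and rock sprite type (plain, steel, gold, diamond) are disconnected.
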(event OnComponentHit(Hit/BlockBox)
  (params (HitComponent :type Primitive%20Component%20Object%20Reference) (OtherActor :type Actor%20Object%20Reference) (OtherComp :type Primitive%20Component%20Object%20Reference) (NormalImpulse :type Vector :default "0, 0, 0") (Hit :type Hit%20Result%20Structure%20%28by%20ref%29))
  (if (== OtherActor (Variables|Default|GetTilemap%20Reference))
    (Physics|SetPhysicsLinearVelocity (Variables|Default|GetRenderComponent) "0, 0, 0" false "None")))

(event EventBeginPlay
  (Utilities|FlowControl|Sequence
    (:then_0
      (bind _aslvl__fuerza_y_velocidad_tilemap_blueprint (Utilities|Casting|CastToLvl-Fuerza_y_velocidad_tilemap_BlueprintClass "/Game/Blueprints/Lvl-Fuerza_y_velocidad_tilemap_Blueprint.Lvl-Fuerza_y_velocidad_tilemap_Blueprint_C"))
      (bind _returnvalue (Actor|GetActorOfClass _aslvl__fuerza_y_velocidad_tilemap_blueprint))
      (Variables|Default|SetTilemap%20Reference _returnvalue))))

(event Collision|EventActorBeginOverlap
  (params (OtherActor :type Actor%20Object%20Reference)))

(event EventTick
  (params (DeltaSeconds :type Float%20%28single-precision%29))
  (bind _returnvalue (Physics|GetPhysicsLinearVelocity (Variables|Default|GetRenderComponent) "None")))

(fn ConstructionScript)