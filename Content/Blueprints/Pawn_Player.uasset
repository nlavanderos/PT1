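; Player pawn for a two-player 2D Paper game, tinted by controller ID.
; Per-player axes move pawns 0 and 1 in the XZ plane, while DireccionMov picks directional flipbooks from player 0's axes alone.
; Holding F on a hit pushes physics objects.
; On the Fuerza_y_velocidad tilemap, Tick saves a pre-hole position and teleports the pawn back after delays, which let spring-launched players pass.
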(event OnComponentHit(Player_Hitbox)
  (params (HitComponent :type Primitive%20Component%20Object%20Reference) (OtherActor :type Actor%20Object%20Reference) (OtherComp :type Primitive%20Component%20Object%20Reference) (NormalImpulse :type Vector :default "0, 0, 0") (Hit :type Hit%20Result%20Structure%20%28by%20ref%29))
  (if (Math|Boolean|ANDBoolean (Class|SceneComponent|IsAnySimulatingPhysics OtherComp) (Class|PrimitiveComponent|IsPhysicsCollisionEnabled OtherComp) (Game|Player|IsInputKeyDown (Game|GetPlayerController 0) "F"))
    (Physics|AddImpulse OtherComp (* (Class|Pawn|GetLastMovementInputVector) 1e+03) "None" false)))

(event EventBeginPlay
  (bind _paperflipbook (Variables|Default|GetPaperFlipbook))
  (Utilities|FlowControl|Sequence
    (:then_0
      (bind _asmultiplayer_gamemode (Utilities|Casting|CastToMultiplayer_Gamemode (Game|GetGameMode)))
      (Variables|Default|SetGamemode _asmultiplayer_gamemode))
    (:then_1
      (bind _aslvl__fuerza_y_velocidad_tilemap_blueprint (Utilities|Casting|CastToLvl-Fuerza_y_velocidad_tilemap_BlueprintClass "/Game/Blueprints/Lvl-Fuerza_y_velocidad_tilemap_Blueprint.Lvl-Fuerza_y_velocidad_tilemap_Blueprint_C"))
      (bind _returnvalue (Actor|GetActorOfClass _aslvl__fuerza_y_velocidad_tilemap_blueprint))
      (Variables|Default|SetTilemap%20Reference _returnvalue))
    (:then_2
      (Utilities|FlowControl|Delay 1e-06)
      (bind _asplayer_controller (Utilities|Casting|CastToPlayerController (Pawn|GetController)))
      (bind _output_get (Variables|Default|SetPlayer%20Controller _asplayer_controller))
      (Utilities|FlowControl|Sequence
        (:then_0
          (switch int (Class|GameplayStatics|GetPlayerControllerID _output_get)
            (:0
              (Sprite|SetSpriteColor _paperflipbook "(R=0.399446,G=0.484375,B=0.020045,A=1.000000)"))
            (:1
              (Sprite|SetSpriteColor _paperflipbook "(R=0.484375,G=0.000000,B=0.044339,A=1.000000)"))))
        (:then_1
          (Input|EnableInput (Variables|Default|GetPlayer%20Controller)))))))

(event Collision|EventActorBeginOverlap
  (params (OtherActor :type Actor%20Object%20Reference)))

(event EventTick
  (params (DeltaSeconds :type Float%20%28single-precision%29))
  (bind _tilemap_reference (Variables|Default|GetTilemap%20Reference))
  (bind _player_hitbox (Variables|Default|GetPlayer_Hitbox))
  (bind _hole (Variables|/Game/Blueprints/Lvl-Fuerza_y_velocidad_tilemap_Blueprint.Lvl-Fuerza_y_velocidad_tilemap_Blueprint_C|GetHole _tilemap_reference))
  (bind _returnvalue (Class|PrimitiveComponent|IsOverlappingComponent _player_hitbox _hole))
  (Utilities|FlowControl|Sequence
    (:then_1
      (if true
        (CallFunction|DireccionMov)))
    (:then_2
      (if (Utilities|Enum|Equal(Enum) (Utilities|GetDisplayName _tilemap_reference) "Lvl-Fuerza_y_velocidad_tilemap_Blueprint")
        ;[1 1 1] Este tiempo deja pasar a los jugadores con el resorte
        (if _returnvalue
          (Utilities|FlowControl|DoOnce false :!label _label
            (:Completed
              (Variables|Default|SetPrevious%20Location (- (- (Transformation|GetActorLocation) (* (Pawn|Components|PawnMovement|GetLastInputVector (Variables|Default|GetFloatingPawnMovement1)) 16.0)) (|Velocity_direction self)))
              (Utilities|FlowControl|Delay 0.2)
              (if _returnvalue
                ;[1 1 1] Mueve al jugador a su posicion antes de tocar el agujero
                (Utilities|FlowControl|Delay 0.2)
                (bind _newparam (CallFunction|PositionDifference))
                (Transformation|SetActorLocation _newparam false true)
                (if _returnvalue
                  (Transformation|SetActorLocation (|Littlemore _newparam) false true)))))
          (else
            (goto _label Reset)))))
    (:then_3)))

(event Input|AxisEvents|InputAxisArriba&abajo(1)
  (params (AxisValue :type Float%20%28single-precision%29))
  (Pawn|Input|AddMovementInput (Game|Player|GetPlayerPawn 1) "0.000000,0.000000,1.000000" AxisValue false))

(event Input|AxisEvents|InputAxisIzquierda&derecha(0)
  (params (AxisValue :type Float%20%28single-precision%29))
  (Pawn|Input|AddMovementInput (Game|Player|GetPlayerPawn 0) "1.000000,0.000000,0.000000" AxisValue false))

(event Input|AxisEvents|InputAxisArriba&abajo(0)
  (params (AxisValue :type Float%20%28single-precision%29))
  (Pawn|Input|AddMovementInput (Game|Player|GetPlayerPawn 0) "0.000000,0.000000,1.000000" AxisValue false))

(event Input|AxisEvents|InputAxisIzquierda&derecha(1)
  (params (AxisValue :type Float%20%28single-precision%29))
  (Pawn|Input|AddMovementInput (Game|Player|GetPlayerPawn 1) "1.000000,0.000000,0.000000" AxisValue false))

(fn ConstructionScript)

(fn DireccionMov
  (bind _paperflipbook (Variables|Default|GetPaperFlipbook))
  (if (or (!= (Input|AxisValues|GetArriba&abajo(0)) 0.0) (!= (Input|AxisValues|GetIzquierda&derecha(0)) 0.0))
    (if (!= (Variables|/Script/Engine.FloatingPawnMovement|GetMaxSpeed (Variables|Default|GetFloatingPawnMovement1)) 0.0)
      (Variables|Default|SetDireccions (select (< (Input|AxisValues|GetIzquierda&derecha(0)) 0.0) "NewEnumerator0" (select (> (Input|AxisValues|GetIzquierda&derecha(0)) 0.0) "NewEnumerator1" (select (> (Input|AxisValues|GetArriba&abajo(0)) 0.0) "NewEnumerator3" "NewEnumerator2"))))
      (Sprite|SetFlipbook _paperflipbook (Utilities|Select :Index (Variables|Default|GetDireccions) :NewEnumerator0 "/Game/Sprites/PJ_sides/LEFT/Left_mov.Left_mov" :NewEnumerator1 "/Game/Sprites/PJ_sides/RIGHT/Right_mov.Right_mov" :NewEnumerator2 "/Game/Sprites/PJ_sides/DOWN/Down_mov.Down_mov" :NewEnumerator3 "/Game/Sprites/PJ_sides/UP/Up_mov.Up_mov"))
      (else
        (Sprite|SetFlipbook _paperflipbook (Utilities|Select :Index (Variables|Default|GetDireccions) :NewEnumerator0 "/Game/Sprites/PJ_sides/LEFT/L_not_mov.L_not_mov" :NewEnumerator1 "/Game/Sprites/PJ_sides/RIGHT/R_not_mov.R_not_mov" :NewEnumerator2 "/Game/Sprites/PJ_sides/DOWN/D_not_mov.D_not_mov" :NewEnumerator3 "/Game/Sprites/PJ_sides/UP/U_not_mov.U_not_mov") :!label _label)))
    (else
      (goto _label))))

(fn PositionDifference
  (bind _returnvalue (Transformation|GetActorLocation))
  (return (- _returnvalue (- _returnvalue (Variables|Default|GetPrevious%20Location)))))