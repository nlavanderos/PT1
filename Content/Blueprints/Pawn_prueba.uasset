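; Test pawn ("prueba") that moves on the X-Z plane and pushes objects it hits.
; Two input axes feed AddMovementInput for left/right and up/down movement.
; On Box hit, it casts the other actor to the Fuerza_y_velocidad tilemap Blueprint and, unless they match, applies an impulse to the hit component along the last movement input.
; An AddForce alternative is left unconnected.
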(event OnComponentHit(Box)
  (params (HitComponent :type Primitive%20Component%20Object%20Reference) (OtherActor :type Actor%20Object%20Reference) (OtherComp :type Primitive%20Component%20Object%20Reference) (NormalImpulse :type Vector :default "0, 0, 0") (Hit :type Hit%20Result%20Structure%20%28by%20ref%29))
  (Utilities|FlowControl|Sequence
    (:then_0
      (bind _aslvl__fuerza_y_velocidad_tilemap_blueprint (Utilities|Casting|CastToLvl-Fuerza_y_velocidad_tilemap_Blueprint OtherActor)))
    (:then_1
      (if (!= OtherActor _aslvl__fuerza_y_velocidad_tilemap_blueprint)
        (Physics|AddImpulse OtherComp (* (Class|Pawn|GetLastMovementInputVector) 1e+03) "None" false)))))

(event EventBeginPlay)

(event Collision|EventActorBeginOverlap
  (params (OtherActor :type Actor%20Object%20Reference)))

(event EventTick
  (params (DeltaSeconds :type Float%20%28single-precision%29)))

(event Input|AxisEvents|InputAxisIzquierda&derecha
  (params (AxisValue :type Float%20%28single-precision%29))
  (Pawn|Input|AddMovementInput "1.000000,0.000000,0.000000" AxisValue false))

(event Input|AxisEvents|InputAxisArriba&abajo
  (params (AxisValue :type Float%20%28single-precision%29))
  (Pawn|Input|AddMovementInput "0.000000,0.000000,1.000000" AxisValue false))

(fn ConstructionScript)