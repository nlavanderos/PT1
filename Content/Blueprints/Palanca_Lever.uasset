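; Player-operated lever that rotates the actor found near its ObjectPosition offset at BeginPlay, or a light source's Arrow component.
; Tick checks the overlapping PawnPlayer: holding Interact freezes movement, while left/right input rotates the target and tilts the lever sprite.
; Rotation costs Gamemode score through delayed deductions.
; Releasing Interact restores speed and fires a DoOnce that resets the sprite, logs rotation totals and player ID via HttpWrite, then clears the totals.
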(event EventBeginPlay
  (Utilities|FlowControl|Delay 1e-05)
  (Utilities|FlowControl|Sequence
    (:then_0
      (bind _outactors (Actor|GetAllActorsOfClass "/Script/Engine.Actor"))
      (for _array_element _outactors
        (if (and (Math|Vector|Equal(Vector) (Transformation|GetActorLocation _array_element) (+ (Transformation|GetActorLocation) (Variables|Default|GetObject%20position)) 3e+01) (!= (Utilities|GetClass _array_element) "/Script/AIModule.AIController"))
          (Variables|Default|SetObject%20to%20control _array_element))))
    (:then_1
      (bind _asmultiplayer_gamemode (Utilities|Casting|CastToMultiplayer_Gamemode (Game|GetGameMode)))
      (bind _output_get (Variables|Default|SetGamemode _asmultiplayer_gamemode))
      (Variables|Default|SetNum%20Players (Utilities|Array|Length (Variables|/Game/Blueprints/Multiplayer_Gamemode.Multiplayer_Gamemode_C|GetPlayers%20 _output_get))))
    (:then_2
      (bind _aslight_source (Utilities|Casting|CastToLight_sourceClass "/Game/Blueprints/Light_source.Light_source_C"))
      (Variables|Default|SetLight_source%20Class _aslight_source))))

(event Collision|EventActorBeginOverlap
  (params (OtherActor :type Actor%20Object%20Reference)))

(event EventTick
  (params (DeltaSeconds :type Float%20%28single-precision%29))
  (bind _gamemode (Variables|Default|GetGamemode))
  (bind _gamemode_2 (Variables|Default|GetGamemode))
  (bind _gamemode_3 (Variables|Default|GetGamemode))
  (bind _object_to_control (Variables|Default|GetObject%20to%20control))
  (bind _gamemode_4 (Variables|Default|GetGamemode))
  (bind _player_detection (Variables|Default|GetPlayer%20Detection))
  (bind _object_to_control_2 (Variables|Default|GetObject%20to%20control))
  (bind _overlappingactors (Collision|GetOverlappingActors _player_detection "/Game/Blueprints/PawnPlayer.PawnPlayer_C" :!class /Script/Engine.PrimitiveComponent))
  (if (Utilities|Array|IsValidIndex _overlappingactors)
    (for _index (range 0 (- (Variables|Default|GetNum%20Players) 1))
      (if (== (Utilities|Array|Get(acopy) _overlappingactors) (Game|Player|GetPlayerPawn _index))
        (Variables|Default|SetPlayer%20ID _index)
        (bind _aspawn_player (Utilities|Casting|CastToPawnPlayer (Game|Player|GetPlayerPawn (Variables|Default|GetPlayer%20ID))))
        (if (Variables|/Game/Blueprints/PawnPlayer.PawnPlayer_C|GetInteract? _aspawn_player)
          (Utilities|FlowControl|Sequence
            (:then_0
              (bind _aspawn_player_2 (Utilities|Casting|CastToPawnPlayer (Game|Player|GetPlayerPawn (Variables|Default|GetPlayer%20ID))))
              (if (!= (Variables|/Game/Blueprints/PawnPlayer.PawnPlayer_C|GetIzq_Der%280%29 _aspawn_player_2) 0.0)
                (if (> (Variables|/Game/Blueprints/PawnPlayer.PawnPlayer_C|GetIzq_Der%280%29 _aspawn_player_2) 0.0)
                  (Utilities|FlowControl|Sequence
                    (:then_0
                      (Utilities|FlowControl|Delay 0.04)
                      (if (== (Utilities|GetClass _object_to_control_2) (Variables|Default|GetLight_source%20Class))
                        (bind _returnvalue (Actor|GetActorOfClass (Variables|Default|GetLight_source%20Class)))
                        (Transformation|AddLocalRotation (Variables|/Game/Blueprints/Light_source.Light_source_C|GetArrow _returnvalue) "0.500000, 0, 0" false false)
                        (Variables|Default|SetRotacion_total%28positiva%29 (+ (Variables|Default|GetRotacion_total%28positiva%29) 0.5))
                        (Utilities|FlowControl|Delay 0.5)
                        (Variables|/Game/Blueprints/Multiplayer_Gamemode.Multiplayer_Gamemode_C|Setscore _gamemode_4 (- (Variables|/Game/Blueprints/Multiplayer_Gamemode.Multiplayer_Gamemode_C|Getscore _gamemode_4) 15))
                        (else
                          (Transformation|AddActorLocalRotation _object_to_control_2 "0.500000,0.0,0.000000" false false)
                          (Variables|Default|SetRotacion_total%28positiva%29 (+ (Variables|Default|GetRotacion_total%28positiva%29) 0.5))
                          (Utilities|FlowControl|Delay 0.5)
                          (Variables|/Game/Blueprints/Multiplayer_Gamemode.Multiplayer_Gamemode_C|Setscore _gamemode_3 (- (Variables|/Game/Blueprints/Multiplayer_Gamemode.Multiplayer_Gamemode_C|Getscore _gamemode_3) 15)))))
                    (:then_1
                      (Rendering|Components|Sprite|SetSprite (Variables|Default|GetPaperSprite) "/Game/Sprites/Palanca/Lever_Sprite.Lever_Sprite")
                      (Transformation|SetRelativeRotation (Variables|Default|GetPaperSprite) "0.000000, 0,3.000000" false false)))
                  (else
                    (Utilities|FlowControl|Sequence
                      (:then_0
                        (Utilities|FlowControl|Delay 0.04)
                        (if (== (Utilities|GetClass _object_to_control) (Variables|Default|GetLight_source%20Class))
                          (bind _returnvalue_2 (Actor|GetActorOfClass (Variables|Default|GetLight_source%20Class)))
                          (Transformation|AddLocalRotation (Variables|/Game/Blueprints/Light_source.Light_source_C|GetArrow _returnvalue_2) "-0.500000, 0, 0" false false)
                          (Variables|Default|SetRotacion_total%28negativa%29 (- (Variables|Default|GetRotacion_total%28negativa%29) 0.5))
                          (Utilities|FlowControl|Delay 0.5)
                          (Variables|/Game/Blueprints/Multiplayer_Gamemode.Multiplayer_Gamemode_C|Setscore _gamemode_2 (- (Variables|/Game/Blueprints/Multiplayer_Gamemode.Multiplayer_Gamemode_C|Getscore _gamemode_2) 15))
                          (else
                            (Transformation|AddActorLocalRotation _object_to_control "-0.500000,0.000000,0.000000" false false)
                            (Variables|Default|SetRotacion_total%28negativa%29 (- (Variables|Default|GetRotacion_total%28negativa%29) 0.5))
                            (Utilities|FlowControl|Delay 0.5)
                            (Variables|/Game/Blueprints/Multiplayer_Gamemode.Multiplayer_Gamemode_C|Setscore _gamemode (- (Variables|/Game/Blueprints/Multiplayer_Gamemode.Multiplayer_Gamemode_C|Getscore _gamemode) 15)))))
                      (:then_1
                        (Rendering|Components|Sprite|SetSprite (Variables|Default|GetPaperSprite) "/Game/Sprites/Palanca/Lever_Sprite.Lever_Sprite")
                        (Transformation|SetRelativeRotation (Variables|Default|GetPaperSprite) "0,180.000000,-3.000000" false false)))))))
            (:then_1
              (Utilities|Casting|CastToPawnPlayer (Game|Player|GetPlayerPawn (Variables|Default|GetPlayer%20ID)))
              (Variables|/Script/Engine.FloatingPawnMovement|SetMaxSpeed (Variables|/Game/Blueprints/PawnPlayer.PawnPlayer_C|GetFloatingPawnMovement1 (stale _aspawn_player_3)) 0.0))
            (:then_2
              (goto _label Reset)))
          (else
            (Utilities|FlowControl|Sequence
              (:then_0
                (bind _aspawn_player_3 (Utilities|Casting|CastToPawnPlayer (Game|Player|GetPlayerPawn (Variables|Default|GetPlayer%20ID))))
                (Variables|/Script/Engine.FloatingPawnMovement|SetMaxSpeed (Variables|/Game/Blueprints/PawnPlayer.PawnPlayer_C|GetFloatingPawnMovement1 _aspawn_player_3) 1e+02))
              (:then_1
                (Utilities|FlowControl|DoOnce false :!label _label
                  (:Completed
                    (Rendering|Components|Sprite|SetSprite (Variables|Default|GetPaperSprite) "/Game/Sprites/Palanca/Lever2_Sprite.Lever2_Sprite")
                    (Default|HttpWrite (Variables|Default|GetGamemode) "1" (Utilities|String|Append (Utilities|GetDisplayName self) "; " (Utilities|GetDisplayName (Variables|Default|GetObject%20to%20control)) "; " "Rotación Total Positiva: " (Utilities|String|ToString(Float) (Variables|Default|GetRotacion_total%28positiva%29)) "; Rotación Total Negativa: " (Utilities|String|ToString(Float) (Variables|Default|GetRotacion_total%28negativa%29)) "; Player " (Utilities|String|ToString(Integer) (Variables|Default|GetPlayer%20ID))))
                    (Variables|Default|SetRotacion_total%28positiva%29 0.0)
                    (Variables|Default|SetRotacion_total%28negativa%29 0.0)))))))))))

(fn ConstructionScript)