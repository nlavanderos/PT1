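; Sign actor with a Densidad widget component that shows only while the player pawn is nearby.
; On BeginPlay it casts the widget to Densidad and sets its Velocidad value according to the actor's display name, for two named sign instances.
; Each Tick it shows the widget if a PawnPlayer overlaps the OverlapBox and hides it otherwise, or whenever the OPEN flag is set.
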(event EventBeginPlay
  (Utilities|FlowControl|Sequence
    (:then_0
      (bind _output_get (Variables|Default|SetWidget (UserInterface|GetUserWidgetObject (Variables|Default|GetWidgetComponent))))
      (bind _asdensidad (Utilities|Casting|CastToDensidad _output_get))
      (switch string (Utilities|GetDisplayName self)
        (:Sign_with_Widget1
          (Variables|/Game/Widgets/Densidad.Densidad_C|SetVelocidad _asdensidad 18.0))
        (:Sign_with_Widget2
          (Variables|/Game/Widgets/Densidad.Densidad_C|SetVelocidad _asdensidad 23.0))))))

(event Collision|EventActorBeginOverlap
  (params (OtherActor :type Actor%20Object%20Reference)))

(event EventTick
  (params (DeltaSeconds :type Float%20%28single-precision%29))
  (bind _widget (Variables|Default|GetWidget))
  (Utilities|FlowControl|Sequence
    (:then_0
      (if (Variables|Default|GetOPEN)
        (Widget|SetVisibility _widget "Hidden")
        (elif (Utilities|Array|IsValidIndex (Collision|GetOverlappingActors (Variables|Default|GetOverlapBox) "/Game/Blueprints/PawnPlayer.PawnPlayer_C" :!class /Script/Engine.PrimitiveComponent))
          (Widget|SetVisibility _widget "Visible")
          (else
            (Widget|SetVisibility _widget "Hidden")))))))

(fn ConstructionScript)