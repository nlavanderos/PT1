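; Paper2D player pawn that moves on the X/Z plane from axis input and pushes physics objects.
; Each Tick, DireccionMov picks a walking flipbook from input, favoring horizontal, or an idle one for the last direction when input or FloatingPawnMovement MaxSpeed is zero.
; UP and DOWN enum values map to oppositely named flipbooks.
; Hitbox hits apply an impulse along the last movement input, excluding the Fuerza_y_velocidad tilemap actor.
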(event OnComponentHit(Player_Hitbox)
  (params (HitComponent :type Primitive%20Component%20Object%20Reference) (OtherActor :type Actor%20Object%20Reference) (OtherComp :type Primitive%20Component%20Object%20Reference) (NormalImpulse :type Vector :default "0, 0, 0") (Hit :type Hit%20Result%20Structure%20%28by%20ref%29))
  (bind _aslvl__fuerza_y_velocidad_tilemap_blueprint (Utilities|Casting|CastToLvl-Fuerza_y_velocidad_tilemap_BlueprintClass "/Game/Blueprints/Lvl-Fuerza_y_velocidad_tilemap_Blueprint.Lvl-Fuerza_y_velocidad_tilemap_Blueprint_C"))
  (bind _returnvalue (Actor|GetActorOfClass _aslvl__fuerza_y_velocidad_tilemap_blueprint))
  (if (and (!= OtherActor _returnvalue) (Class|SceneComponent|IsAnySimulatingPhysics (Variables|/Script/Engine.Actor|GetRootComponent OtherActor)))
    (Physics|AddImpulse OtherComp (* (Class|Pawn|GetLastMovementInputVector) 1e+03) "None" false)))

(event EventBeginPlay)

(event Collision|EventActorBeginOverlap
  (params (OtherActor :type Actor%20Object%20Reference)))

(event EventTick
  (params (DeltaSeconds :type Float%20%28single-precision%29))
  (Utilities|FlowControl|Sequence
    (:then_0
      (CallFunction|DireccionMov))))

(event Input|AxisEvents|InputAxisIzquierda&derecha
  (params (AxisValue :type Float%20%28single-precision%29))
  (Pawn|Input|AddMovementInput "1.000000,0.000000,0.000000" AxisValue false))

(event Input|AxisEvents|InputAxisArriba&abajo
  (params (AxisValue :type Float%20%28single-precision%29))
  (Pawn|Input|AddMovementInput "0.000000,0.000000,1.000000" AxisValue false))

(fn ConstructionScript)

(fn DireccionMov
  (bind _paperflipbook (Variables|Default|GetPaperFlipbook))
  (if (or (!= (Input|AxisValues|GetArriba&abajo) 0.0) (!= (Input|AxisValues|GetIzquierda&derecha) 0.0))
    (if (!= (Variables|/Script/Engine.FloatingPawnMovement|GetMaxSpeed (Variables|Default|GetFloatingPawnMovement1)) 0.0)
      (Variables|Default|SetDireccions (select (< (Input|AxisValues|GetIzquierda&derecha) 0.0) "NewEnumerator0" (select (> (Input|AxisValues|GetIzquierda&derecha) 0.0) "NewEnumerator1" (select (> (Input|AxisValues|GetArriba&abajo) 0.0) "NewEnumerator3" "NewEnumerator2"))))
      (Sprite|SetFlipbook _paperflipbook (Utilities|Select :Index (Variables|Default|GetDireccions) :NewEnumerator0 "/Game/Sprites/PJ_sides/LEFT/Left_mov.Left_mov" :NewEnumerator1 "/Game/Sprites/PJ_sides/RIGHT/Right_mov.Right_mov" :NewEnumerator2 "/Game/Sprites/PJ_sides/DOWN/Down_mov.Down_mov" :NewEnumerator3 "/Game/Sprites/PJ_sides/UP/Up_mov.Up_mov"))
      (else
        (Sprite|SetFlipbook _paperflipbook (Utilities|Select :Index (Variables|Default|GetDireccions) :NewEnumerator0 "/Game/Sprites/PJ_sides/LEFT/L_not_mov.L_not_mov" :NewEnumerator1 "/Game/Sprites/PJ_sides/RIGHT/R_not_mov.R_not_mov" :NewEnumerator2 "/Game/Sprites/PJ_sides/DOWN/D_not_mov.D_not_mov" :NewEnumerator3 "/Game/Sprites/PJ_sides/UP/U_not_mov.U_not_mov") :!label _label)))
    (else
      (goto _label))))