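; Local multiplayer game mode that spawns players at index-tagged PlayerStarts and runs each tilemap level through scoring to the next.
; BeginPlay sets camera zoom by player count, creates timer and score widgets, and finds the level index.
; Tick polls players standing on doors in the first two levels, plus broken-door tiles in the first, which freeze the timer.
; Once all players qualify, it animates the score, saves results to GameInstance and opens the next level.
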(event EventBeginPlay
  (bind _players_ (Variables|Default|GetPlayers%20))
  (Utilities|FlowControl|Sequence
    (:then_0
      (CallFunction|PlayersSetSpawns))
    (:then_1
      (if (Utilities|Array|IsValidIndex _players_)
        (for _array_element _players_
          (bind _aspawn_player (Utilities|Casting|CastToPawnPlayer _array_element))
          (bind _asplayer_controller (Utilities|Casting|CastToPlayerController (Pawn|GetController _aspawn_player)))
          (bind _returnvalue (UserInterface|CreateWidget "/Game/Widgets/Tiempo.Tiempo_C" _asplayer_controller))
          (bind _output_get (Variables|Default|SettiempoWid _returnvalue))
          (UserInterface|Viewport|AddtoPlayerScreen _output_get)
          (Widget|SetVisibility _output_get "Hidden"))))
    (:then_2
      (bind _returnvalue_2 (UserInterface|CreateWidget "/Game/Widgets/Puntuacion.Puntuacion_C"))
      (bind _output_get_2 (Variables|Default|SetPuntuacionWidget _returnvalue_2))
      (UserInterface|Viewport|AddtoViewport _output_get_2 0)
      (Widget|SetVisibility _output_get_2 "Hidden"))
    (:then_3
      (bind _asmy_game_instance (Utilities|Casting|CastToMyGameInstance (Game|GetGameInstance)))
      (bind _output_get_3 (Variables|Default|SetGame%20Instance _asmy_game_instance))
      (for (_array_element_2 _array_index) (Variables|/Game/Blueprints/MyGameInstance.MyGameInstance_C|GetLevels _output_get_3)
        (bind _returnvalue_3 (Game|GetCurrentLevelName true))
        (if (Utilities|Enum|Equal(Enum) _array_element_2 _returnvalue_3)
          (Variables|Default|SetLvl%20index _array_index))))))

(event EventTick
  (params (DeltaSeconds :type Float%20%28single-precision%29))
  (bind _returnvalue (Utilities|Time|GetGameTimeinSeconds))
  (bind _fade_movement_discount (Variables|Default|GetFade/Movement_Discount))
  (bind _players_ (Variables|Default|GetPlayers%20))
  (bind _returnvalue_2 (- _returnvalue _fade_movement_discount))
  (bind _returnvalue_3 (Math|Timespan|FromSeconds _returnvalue_2))
  (Utilities|FlowControl|Sequence
    (:then_0
      (if (not (Variables|Default|GetAll%20true%28doors%20broken%29))
        (Variables|Default|SettimeSec (.seconds _returnvalue_3))
        (Variables|Default|SettimeMin (.minutes _returnvalue_3))))
    (:then_1
      (switch int (Variables|Default|GetLvl%20index)
        (:0
          (bind _returnvalue_4 (Actor|GetActorOfClass "/Game/Blueprints/Lvl-Densidad-tilemap_Blueprint.Lvl-Densidad-tilemap_Blueprint_C"))
          (Variables|Default|SetcurrentTileMap _returnvalue_4)
          (Utilities|FlowControl|Sequence
            (:then_0
              (|Door(s)_Broken?(Lv1) (Variables|/Game/Blueprints/Lvl-Densidad-tilemap_Blueprint.Lvl-Densidad-tilemap_Blueprint_C|GetDoors%20to%20break _returnvalue_4)))
            (:then_1
              (|Players_on_Door_Comprobation(Lv1) (Variables|/Game/Blueprints/Lvl-Densidad-tilemap_Blueprint.Lvl-Densidad-tilemap_Blueprint_C|GetDoors%20to%20break _returnvalue_4) _players_))
            (:then_2
              (if (== (Utilities|Array|Length (Variables|Default|GetPlayers%20)) (Utilities|Map|Length (Variables|Default|GetPlayers_on_door))) :!label _label
                (Utilities|FlowControl|Delay (Variables|Default|GetDelay%20at%20end))
                (Utilities|FlowControl|Sequence
                  (:then_0
                    (Utilities|FlowControl|DoOnce false
                      (:Completed
                        (bind _output_get (Variables|Default|SetScore%20init (Variables|Default|Getscore)))
                        (bind _output_get_2 (Variables|Default|SetScore%20end (|Score_on_time)))
                        (bind _foundwidgets (Widget|GetAllWidgetsOfClass "/Game/Widgets/Tiempo.Tiempo_C" true))
                        (if (Utilities|Array|IsValidIndex _foundwidgets)
                          (for _array_element _foundwidgets
                            (Widget|RemovefromParent _array_element)))
                        (Widget|SetVisibility (Variables|Default|GetPuntuacionWidget) "Visible")
                        (bind _score_track (Timeline|Score_Update PlayFromStart)
                          (:Update
                            (Variables|Default|Setscore (Math|Float|Truncate (Math|Float|Lerp (Math|Conversions|ToFloat(Integer) _output_get) (Math|Conversions|ToFloat(Integer) _output_get_2) _score_track))))
                          (:Finished
                            (Variables|/Game/Blueprints/MyGameInstance.MyGameInstance_C|SetCurrent_Session_Score (Variables|Default|GetGame%20Instance) (Variables|Default|GetScore%20end))
                            (Widget|SetVisibility (Variables|Default|GetPuntuacionWidget) "Hidden")
                            (Game|OpenLevel(byName) (Utilities|String|StringToName (Utilities|Array|Get(acopy) (Variables|/Game/Blueprints/MyGameInstance.MyGameInstance_C|GetLevels (Variables|Default|GetGame%20Instance)) (+ (Variables|Default|GetLvl%20index) 1)))))))))
                  (:then_1
                    (Utilities|FlowControl|DoOnce false
                      (:Completed
                        (Variables|/Game/Blueprints/MyGameInstance.MyGameInstance_C|SetCurrent_Session_Time (Variables|Default|GetGame%20Instance) (+ (Variables|Default|GettimeSec) (* (Variables|Default|GettimeMin) 60)))))))))))
        (:1
          (bind _returnvalue_5 (Actor|GetActorOfClass "/Game/Blueprints/Lvl-Fuerza_y_velocidad_tilemap_Blueprint.Lvl-Fuerza_y_velocidad_tilemap_Blueprint_C"))
          (Variables|Default|SetcurrentTileMap _returnvalue_5)
          (Utilities|FlowControl|Sequence
            (:then_0
              (|Players_on_Door_Comprobation(Lv2) (Variables|/Game/Blueprints/Lvl-Fuerza_y_velocidad_tilemap_Blueprint.Lvl-Fuerza_y_velocidad_tilemap_Blueprint_C|GetDoors%20to%20break _returnvalue_5) _players_))
            (:then_2
              (goto _label))))
        (:2
          (bind _returnvalue_6 (Actor|GetActorOfClass "/Script/Paper2D.PaperTileMapActor" :!label _label_2))
          (Variables|Default|SetcurrentTileMap _returnvalue_6))
        (:3
          (goto _label_2))))
    (:then_2
      (Utilities|FlowControl|Delay 0.001)
      (Variables|Default|Setscore_aux (Variables|Default|Getscore)))))

(fn ConstructionScript)

(fn PlayersSetSpawns
  (Utilities|FlowControl|Sequence
    (:then_0
      (bind _outactors (Actor|GetAllActorsOfClass "/Script/Engine.PlayerStart"))
      (LocalVariables|SetSpawn_Points _outactors))
    (:then_1
      (for _index (range 0 (- (Variables|Default|GetMax_Players) 1))
        (LocalVariables|SetIndex _index)
        (for _array_element (LocalVariables|GetSpawn_Points)
          (if (Utilities|Name|Equal(Name) (Variables|/Script/Engine.PlayerStart|GetPlayerStartTag _array_element) (Utilities|String|StringToName (Utilities|String|ToString(Integer) (LocalVariables|GetIndex))))
            (bind _returnvalue (Class|GameplayStatics|CreatePlayer (LocalVariables|GetIndex)))
            (LocalVariables|SetPlayer%20Controller _returnvalue)
            (LocalVariables|SetPlayer_start_transform (Transformation|GetActorTransform _array_element))
            (|Index() 0 (LocalVariables|GetPlayer_start_transform))))
        (bind _returnvalue_2 (Game|GetCurrentLevelName true))
        (switch int (- (Variables|Default|GetMax_Players) 1)
          (:0
            (if (Utilities|Enum|Equal(Enum) _returnvalue_2 "Densidad_de_Objetos")
              (LocalVariables|SetCamera%20Zoom 4e+02)
              (else
                (LocalVariables|SetCamera%20Zoom 4e+02))))
          (:1
            (LocalVariables|SetCamera%20Zoom 3e+02)))
        (for _array_element_2 (Variables|Default|GetPlayers%20)
          (bind _aspawn_player (Utilities|Casting|CastToPawnPlayer _array_element_2))
          (Class|CameraComponent|SetOrthoWidth (Variables|/Game/Blueprints/PawnPlayer.PawnPlayer_C|GetPlayer_Camera _aspawn_player) (LocalVariables|GetCamera%20Zoom)))))))

(fn FindElementonTilemap(X)
  (params (Vector :type Vector%20%28by%20ref%29) (Integer :type Integer) (Tilemap :type Paper%20Tile%20Map%20Actor%20Object%20Reference))
  (bind _rendercomponent (Variables|/Script/Paper2D.PaperTileMapActor|GetRenderComponent Tilemap))
  (bind _tilemap (Variables|/Script/Paper2D.PaperTileMapComponent|GetTileMap _rendercomponent))
  (bind _output_get (LocalVariables|SetLocal%20Vector%28Find%29 Vector))
  (LocalVariables|SetLast%20Layer Integer)
  (bind _index (Utilities|FlowControl|ForLoopwithBreak 0 (- (Variables|/Script/Paper2D.PaperTileMap|GetMapWidth _tilemap) 1) :!label _label)
    (:LoopBody
      (LocalVariables|SetX%28N%29 _index)
      (bind _index_2 (Utilities|FlowControl|ForLoopwithBreak 0 (- (Variables|/Script/Paper2D.PaperTileMap|GetMapHeight _tilemap) 1))
        (:LoopBody
          (LocalVariables|SetY%28N%29 _index_2)
          (if (Math|Vector|Equal(Vector) _output_get (Class|PaperTileMapComponent|GetTileCenterPosition (Variables|/Script/Paper2D.PaperTileMapActor|GetRenderComponent Tilemap) (LocalVariables|GetX%28N%29) (LocalVariables|GetY%28N%29) (LocalVariables|GetLast%20Layer) true) 16.0)
            (Utilities|FlowControl|Sequence
              (:then_0
                (bind _output_get_2 (LocalVariables|SetX%28N%29%28aux%29 (LocalVariables|GetX%28N%29)))
                (bind _output_get_3 (LocalVariables|SetY%28N%29%28aux%29 (LocalVariables|GetY%28N%29)))
                (return _output_get_2 _output_get_3))
              (:then_1
                (goto _label Break)))))))))