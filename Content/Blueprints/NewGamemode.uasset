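; Game mode that keeps an elapsed minutes-and-seconds timer and zeroes the score on the first tick.
; Tick checks the P flag on the Fuerza y velocidad tilemap actor: false feeds an open Gate, true closes it for good.
; The Gate drives a one-second Delay that increments the seconds and rolls them into minutes.
; BeginPlay creates the Tiempo widget, but its AddToViewport call is never executed.
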(event EventBeginPlay
  (bind _returnvalue (UserInterface|CreateWidget "/Game/Blueprints/Tiempo.Tiempo_C"))
  (bind _output_get (Variables|Default|SettiempoWid _returnvalue)))

(event EventTick
  (params (DeltaSeconds :type Float%20%28single-precision%29))
  (Utilities|FlowControl|Sequence
    (:then_0
      (if (Utilities|IsValid (stale _returnvalue))
        (bind _aslvl__fuerza_y_velocidad_tilemap_blueprint (Utilities|Casting|CastToLvl-Fuerza_y_velocidad_tilemap_BlueprintClass "/Game/Blueprints/Lvl-Fuerza_y_velocidad_tilemap_Blueprint.Lvl-Fuerza_y_velocidad_tilemap_Blueprint_C"))
        (bind _returnvalue (Actor|GetActorOfClass _aslvl__fuerza_y_velocidad_tilemap_blueprint))
        (if (Variables|/Game/Blueprints/Lvl-Fuerza_y_velocidad_tilemap_Blueprint.Lvl-Fuerza_y_velocidad_tilemap_Blueprint_C|Getp _returnvalue)
          (goto _label Close)
          (else
            (Utilities|FlowControl|Gate false :!label _label
              (:Exit
                (Utilities|FlowControl|Delay 1.0)
                (Variables|Default|SettimeSec (+ (Variables|Default|GettimeSec) 1))
                (if (> (Variables|Default|GettimeSec) 59)
                  (Variables|Default|SettimeMin (+ (Variables|Default|GettimeMin) 1))
                  (Variables|Default|SettimeSec 0))))))))
    (:then_1
      (Utilities|FlowControl|DoOnce false
        (:Completed
          (Variables|Default|Setscore 0))))))

(fn ConstructionScript)